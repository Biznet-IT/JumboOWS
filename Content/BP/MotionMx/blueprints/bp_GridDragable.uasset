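; Editable grid of draggable point actors, whose saved layout the comments tie to a Warp configuration.
; Construction script and Init spawn bp_GridDragablePoint child actors per cell corner, with Init restoring supplied world positions if the count matches.
; Clicking grabs a point, and Tick moves it to the cursor's trace hit on the PlaneGridBg background plane.
; Release or cursor exit ends dragging and fires OnGridUpdated; ObtenerPuntos returns all world positions.
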(event Custom|Init
  (params (TotalColumnas :type Integer) (TotalFilas :type Integer) (GridWidth :type Integer) (GridHeight :type Integer) (Points :type Array%20of%20Vectors))
  (bind _returnvalue (Utilities|Array|Length Points))
  (Variables|Default|SetTotalColumnas TotalColumnas)
  (Variables|Default|SetTotalFilas TotalFilas)
  (Variables|Default|SetGridWidth GridWidth)
  (Variables|Default|SetGridHeight GridHeight)
  (if (or (!= (* (+ (Variables|Default|GetTotalColumnas) 1) (+ (Variables|Default|GetTotalFilas) 1)) _returnvalue) (< _returnvalue 4))
    (Utilities|Array|Clear (Variables|Default|GetPreExistingPoints))
    (else
      (Variables|Default|SetPreExistingPoints Points)))
  (Utilities|FlowControl|Sequence
    (:then_0
      (CallFunction|RemoveAllDragablePoints))
    (:then_1
      ;[1 0.2887 0.07785] calcular ancho y alto de cada celda
      (Variables|Default|SetcellWidth (/ (Math|Conversions|ToFloat(Integer) (Variables|Default|GetGridWidth)) (Math|Conversions|ToFloat(Integer) (Variables|Default|GetTotalColumnas))))
      (Variables|Default|SetcellHeight (/ (Math|Conversions|ToFloat(Integer) (Variables|Default|GetGridHeight)) (Math|Conversions|ToFloat(Integer) (Variables|Default|GetTotalFilas)))))
    (:then_2
      ;[0 0.1996 0.2865] crear cada punto de la cuadricula
      (for _index (range 0 (Variables|Default|GetTotalFilas))
        (for _index_2 (range 0 (Variables|Default|GetTotalColumnas))
          (bind _returnvalue_2 (AddComponent|AddChildActorComponent false))
          (bind _output_get (Variables|Default|SetChildActor_tmp _returnvalue_2))
          (ChildActorComponent|SetChildActorClass _output_get "/Game/BP/MotionMx/blueprints/bp_GridDragablePoint.bp_GridDragablePoint_C")
          (if (== (Utilities|Array|Length (Variables|Default|GetPreExistingPoints)) 0)
            (Transformation|SetRelativeLocation (Variables|Default|GetChildActor_tmp) (Math|Vector|MakeVector (* _index_2 (Variables|Default|GetcellWidth)) (.y (Variables|/Script/Engine.SceneComponent|GetRelativeLocation (Variables|Default|GetPlaneGridBg))) (* (* _index (Variables|Default|GetcellHeight)) -1.0)) false false) ; 5 en Y para que no golpee el plano verde (tiene fisicas para obtener posicion del mouse)
            (else
              (Transformation|SetWorldLocation (Variables|Default|GetChildActor_tmp) (Utilities|Array|Get(acopy) (Variables|Default|GetPreExistingPoints) (Utilities|Array|Length (Variables|Default|GetAllDragablePoints))) false false) ; aqui uso posiciones de world porque cuando guardo\nconfiguracion Warp en disco asi se almacenan (world locations)
            ))
          (bind _asbp_grid_dragable_point (Utilities|Casting|CastTobp_GridDragablePoint (Variables|/Script/Engine.ChildActorComponent|GetChildActor (Variables|Default|GetChildActor_tmp))))
          ;[1 0.8739 0] agregar listeners de mouse al punto recien creado
          (EventDispatchers|BindEventtoOnClicked _asbp_grid_dragable_point (delegate Custom|onPointClick))
          (EventDispatchers|BindEventtoOnReleased _asbp_grid_dragable_point (delegate Custom|onPointRelease))
          (EventDispatchers|BindEventtoOnEndCursorOver _asbp_grid_dragable_point (delegate Custom|onEndMouseOver))
          ;[0 0 0] agregar punto al array
          (Utilities|Array|Add (Variables|Default|GetAllDragablePoints) _asbp_grid_dragable_point))))))

(event Custom|onDragFinish
  (params (Point%20to%20set :type Bp%20Grid%20Dragable%20Point%20Object%20Reference))
  ;[1 0.3958 0.9892] Drag FINISH
  (Variables|Default|SetPointDragged 0)
  (Default|CallOnGridUpdated))

(event Custom|RemoveAllDragablePoints
  ;[0 0 0 1 15] clear points
  (for _array_element (Variables|Default|GetAllDragablePoints)
    (Components|DestroyComponent (Class|Actor|GetParentComponent _array_element)))
  (Utilities|Array|Clear (Variables|Default|GetAllDragablePoints)))

(event Custom|onPointClick
  (params (TouchedActor :type Actor%20Object%20Reference) (ButtonPressed :type Key%20Structure :default "None"))
  ;[1 0.8739 0] agregar listeners de mouse al punto recien creado
  (bind _asbp_grid_dragable_point (Utilities|Casting|CastTobp_GridDragablePoint TouchedActor))
  (Variables|Default|SetPointDragged _asbp_grid_dragable_point))

(event Custom|onPointRelease
  (params (TouchedActor :type Actor%20Object%20Reference) (ButtonReleased :type Key%20Structure :default "None"))
  ;[1 0.8739 0] agregar listeners de mouse al punto recien creado
  (CallFunction|OnDragFinish))

(event Custom|onEndMouseOver
  (params (TouchedActor :type Actor%20Object%20Reference))
  ;[1 0.8739 0] agregar listeners de mouse al punto recien creado
  (CallFunction|OnDragFinish))

(event EventTick
  (params (DeltaSeconds :type Float%20%28single-precision%29))
  (bind _returnvalue (Game|GetPlayerController 0))
  (bind _hitresult (Game|Player|GetHitResultUnderCursorbyChannel _returnvalue "TraceTypeQuery1" true))
  (Utilities|FlowControl|Sequence
    (:then_0
      ;[1 0.3797 0.8872] Jalar punto con mouse,  uso el plano BG para obtener la posicion del mouse 3d
      (Utilities|IsValid (Variables|Default|GetPointDragged)
        (:Is%20Valid
          (if (Utilities|Enum|Equal(Enum) (Utilities|GetObjectName (.hitcomponent _hitresult)) (Utilities|GetObjectName (Variables|Default|GetPlaneGridBg)))
            (Transformation|SetActorLocation (Variables|Default|GetPointDragged) (.impactpoint _hitresult) false false)))))))

(fn ConstructionScript
  (Utilities|FlowControl|Sequence
    (:then_0
      (Variables|Default|SetcellWidth (/ (Math|Conversions|ToFloat(Integer) (Variables|Default|GetGridWidth)) (Math|Conversions|ToFloat(Integer) (Variables|Default|GetTotalColumnas))))
      (Variables|Default|SetcellHeight (/ (Math|Conversions|ToFloat(Integer) (Variables|Default|GetGridHeight)) (Math|Conversions|ToFloat(Integer) (Variables|Default|GetTotalFilas)))))
    (:then_1
      (for _index (range 0 (Variables|Default|GetTotalFilas))
        (for _index_2 (range 0 (Variables|Default|GetTotalColumnas))
          (bind _returnvalue (AddComponent|AddChildActorComponent false))
          (bind _output_get (Variables|Default|SetChildActor_tmp _returnvalue))
          (ChildActorComponent|SetChildActorClass _output_get "/Game/BP/MotionMx/blueprints/bp_GridDragablePoint.bp_GridDragablePoint_C")
          (Transformation|SetRelativeLocation (Variables|Default|GetChildActor_tmp) (Math|Vector|MakeVector (* _index_2 (Variables|Default|GetcellWidth)) 0.0 (* (* _index (Variables|Default|GetcellHeight)) -1.0)) false false)
          (bind _asbp_grid_dragable_point (Utilities|Casting|CastTobp_GridDragablePoint (Variables|/Script/Engine.ChildActorComponent|GetChildActor (Variables|Default|GetChildActor_tmp))))
          (Utilities|Array|Add (Variables|Default|GetAllDragablePoints) _asbp_grid_dragable_point))))))

(fn ObtenerPuntos
  (for _array_element (Variables|Default|GetAllDragablePoints)
    (Utilities|Array|Add (LocalVariables|GetArray) (Transformation|GetWorldLocation (Variables|/Script/Engine.Actor|GetRootComponent _array_element))))
  (return (LocalVariables|GetArray)))