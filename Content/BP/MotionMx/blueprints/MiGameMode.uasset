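; MiGameMode is a game mode Blueprint that numbers players as they join.
; On PostLogin, with authority, it casts the new controller to MiPlayerController, passes it the current PlayerCount as its player index, then increments the count.
; Debug strings report each login or a failed cast, and an older path that set index zero and called CallOnIndex is left unconnected.
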(event EventPostLogin
  (params (NewPlayer :type Player%20Controller%20Object%20Reference))
  (Networking|SwitchHasAuthority
    (:Authority
      (bind _asmi_player_controller (Utilities|Casting|CastToMiPlayerController NewPlayer)
        (:then
          (Development|PrintString (Utilities|String|Append "on Post login : " (Utilities|GetDisplayName NewPlayer)) true true "(R=0.000000,G=1.000000,B=0.070817,A=1.000000)" 5.0)
          (if (!= (Variables|Default|GetplayerCount) 0)
            _
            (else
              _))
          (Default|SetPlayerIndex _asmi_player_controller (Variables|Default|GetplayerCount))
          (Math|Integer|IncrementInt (Variables|Default|GetplayerCount)))
        (:CastFailed
          (Development|PrintString "ERROR -> failed to create player controller index" true true "(R=1.000000,G=0.000000,B=0.541865,A=1.000000)" 2e+01))))))

(fn ConstructionScript)