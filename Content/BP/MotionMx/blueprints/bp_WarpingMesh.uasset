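; Warping mesh actor that draws a deformable grid of camera-material quads from world-space control points, with edge gradient blending and HSB adjustment.
; UpdateGrid rebuilds one procedural mesh section per cell in local space, offset behind the draggable points.
; Each cell's dynamic material receives its row, column and grid size, and is stored so UpdateMaterials1 can change gradients and HSB without rebuilding.
; The construction script creates a preview quad, cleared on BeginPlay.
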(event Custom|UpdateGrid
  (params (GridPoints :type Array%20of%20Vectors) (TotalColumnas :type Integer) (TotalFilas :type Integer) (GradientsBlend :type Array%20of%20Vector%202D%20Structures) (HSV :type Array%20of%20Floats%20%28double-precision%29))
  (bind _returnvalue (Transformation|GetActorTransform))
  (Utilities|FlowControl|Sequence
    (:then_0
      (CallFunction|ClearMeshes)
      (Variables|Default|SetMeshSectionIndex 0)
      (Variables|Default|SetTotalColumnas TotalColumnas)
      (Variables|Default|SetTotalFilas TotalFilas)
      (Variables|Default|SetGradients GradientsBlend)
      (Variables|Default|SetHSB HSV))
    (:then_1
      ;[0.1406 0.009966 0.05277 1 15] obtener esquina superior izquierda de cada celda del grid
      (for _index (range 0 (- (Variables|Default|GetTotalFilas) 1))
        (for _index_2 (range 0 (- (Variables|Default|GetTotalColumnas) 1))
          (bind (_tl _tr _bl _br) (CallFunction|ObtenerCuadro (- (+ _index_2 (+ (* _index (+ (Variables|Default|GetTotalColumnas) 1)) 1)) 1) (Variables|Default|GetTotalColumnas)))
          (CallFunction|CrearSeccionMesh (Variables|Default|GetMeshSectionIndex) (Utilities|Array|MakeArray (+ (Math|Transform|InverseTransformLocation _returnvalue (Utilities|Array|Get(acopy) GridPoints _tl)) "2.000000,0.000000,0.000000") (+ (Math|Transform|InverseTransformLocation _returnvalue (Utilities|Array|Get(acopy) GridPoints _bl)) "2.000000,0.000000,0.000000") (+ (Math|Transform|InverseTransformLocation _returnvalue (Utilities|Array|Get(acopy) GridPoints _tr)) "2.000000,0.000000,0.000000") (+ (Math|Transform|InverseTransformLocation _returnvalue (Utilities|Array|Get(acopy) GridPoints _br)) "2.000000,0.000000,0.000000")))
          (bind _returnvalue_2 (Rendering|Material|CreateDynamicMaterialInstance (Variables|Default|GetProceduralMesh) (Variables|Default|GetMeshSectionIndex) "/Game/materiales/mat_camaraSeccionBand_Inst.mat_camaraSeccionBand_Inst" "None" :!class /Script/Engine.PrimitiveComponent))
          (bind _output_get (Variables|Default|SetmaterialTmp _returnvalue_2))
          (Utilities|Array|Add (Variables|Default|Getmateriales) (Utilities|Struct|Makestruct_WarpMeshMaterialProps 0 _output_get (Variables|Default|GetTotalColumnas) (Variables|Default|GetTotalFilas) _index_2 _index (Variables|Default|GetGradients) (Variables|Default|GetHSB)))
          (CallFunction|PropiedadesDeMaterial _output_get (Math|Conversions|ToFloat(Integer) (Variables|Default|GetTotalColumnas)) (Math|Conversions|ToFloat(Integer) (Variables|Default|GetTotalFilas)) (Math|Conversions|ToFloat(Integer) _index_2) (Math|Conversions|ToFloat(Integer) _index) (Variables|Default|GetGradients) (Variables|Default|GetHSB))
          (Math|Integer|IncrementInt (Variables|Default|GetMeshSectionIndex)))))))

(event Custom|clearMeshes
  ;[0 0.1165 0.2656 1 15] clear meshes
  (Class|ProceduralMeshComponent|ClearAllMeshSections (Variables|Default|GetProceduralMesh))
  (Utilities|Array|Clear (Variables|Default|Getmateriales)))

(event Custom|UpdateMaterials1
  (params (Gradients :type Array%20of%20Vector%202D%20Structures) (HSB :type Array%20of%20Floats%20%28double-precision%29))
  (Variables|Default|SetGradients Gradients)
  (Variables|Default|SetHSB HSB)
  (for (_array_element _array_index) (Variables|Default|Getmateriales)
    (Utilities|Array|SetArrayElem (Variables|Default|Getmateriales) _array_index (Utilities|Struct|Makestruct_WarpMeshMaterialProps (.MeshIndex (Utilities|Struct|Breakstruct_WarpMeshMaterialProps _array_element)) (.mat (Utilities|Struct|Breakstruct_WarpMeshMaterialProps _array_element)) (.totalCols (Utilities|Struct|Breakstruct_WarpMeshMaterialProps _array_element)) (.TotalRows (Utilities|Struct|Breakstruct_WarpMeshMaterialProps _array_element)) (.Col (Utilities|Struct|Breakstruct_WarpMeshMaterialProps _array_element)) (.Row (Utilities|Struct|Breakstruct_WarpMeshMaterialProps _array_element)) (Variables|Default|GetGradients) (Variables|Default|GetHSB)))
    (CallFunction|PropiedadesDeMaterial (.mat (Utilities|Struct|Breakstruct_WarpMeshMaterialProps _array_element)) (Math|Conversions|ToFloat(Integer) (.totalCols (Utilities|Struct|Breakstruct_WarpMeshMaterialProps _array_element))) (Math|Conversions|ToFloat(Integer) (.TotalRows (Utilities|Struct|Breakstruct_WarpMeshMaterialProps _array_element))) (Math|Conversions|ToFloat(Integer) (.Col (Utilities|Struct|Breakstruct_WarpMeshMaterialProps _array_element))) (Math|Conversions|ToFloat(Integer) (.Row (Utilities|Struct|Breakstruct_WarpMeshMaterialProps _array_element))) (Variables|Default|GetGradients) (Variables|Default|GetHSB))))

(event EventBeginPlay
  (Utilities|FlowControl|Sequence
    (:then_0
      ;[0 0 0 1 12] limpiar los que cree en tiempo de edicion
      (CallFunction|ClearMeshes))))

(fn ConstructionScript
  (bind _returnvalue (Math|Float|MakeLiteralFloat 0.0))
  (bind _returnvalue_2 (Math|Float|MakeLiteralFloat 1.0))
  (CallFunction|CrearSeccionMesh (LocalVariables|GetMeshSectionIndex) (Utilities|Array|MakeArray "0, 0, 0" "0,100.000000,0.000000" "100.000000,0.000000, 0" "100.000000,100.000000, 0"))
  (bind _returnvalue_3 (Rendering|Material|CreateDynamicMaterialInstance (Variables|Default|GetProceduralMesh) 0 "/Game/materiales/mat_camaraSeccionBand_Inst.mat_camaraSeccionBand_Inst" "None" :!class /Script/Engine.PrimitiveComponent))
  (bind _output_get (LocalVariables|SetmaterialTmp _returnvalue_3))
  (CallFunction|PropiedadesDeMaterial _output_get _returnvalue_2 _returnvalue_2 _returnvalue _returnvalue (Utilities|Array|MakeArray "" "" "" "") (Utilities|Array|MakeArray 1.0 0.0 1.0)))

(fn CrearSeccionMesh
  (params (SeccionIndex :type Integer) (Vertices :type Array%20of%20Vectors))
  (Class|ProceduralMeshComponent|CreateMeshSectionLinearColor (Variables|Default|GetProceduralMesh) SeccionIndex Vertices (Utilities|Array|MakeArray 0 1 2 3 2 1) 0 (Utilities|Array|MakeArray "" "(X=0.000000,Y=1.000000)" "(X=1.000000,Y=0.000000)" "(X=1.000000,Y=1.000000)") 0 0 0 0 0 false))

(fn ObtenerCuadro
  (params (esquinaTL :type Integer) (totalColumnas :type Integer))
  (bind _returnvalue (+ totalColumnas 1))
  (bind _returnvalue_2 (+ esquinaTL _returnvalue))
  (return esquinaTL (+ esquinaTL 1) _returnvalue_2 (+ _returnvalue_2 1)))

(fn PropiedadesDeMaterial
  (params (material :type Material%20Instance%20Dynamic%20Object%20Reference%20%28by%20ref%29) (totalColumnas :type Float%20%28double-precision%29%20%28by%20ref%29) (totalFilas :type Float%20%28double-precision%29%20%28by%20ref%29) (columna :type Float%20%28double-precision%29%20%28by%20ref%29) (fila :type Float%20%28double-precision%29%20%28by%20ref%29) (Gradients :type Array%20of%20Vector%202D%20Structures) (HSB :type Array%20of%20Floats%20%28double-precision%29))
  (bind _output (Utilities|Array|Get(acopy) Gradients 3))
  (bind _output_2 (Utilities|Array|Get(acopy) Gradients))
  (bind _output_3 (Utilities|Array|Get(acopy) Gradients 1))
  (bind _output_4 (Utilities|Array|Get(acopy) Gradients 2))
  (Rendering|Material|SetScalarParameterValue material "TotalColumnas" totalColumnas :!class /Script/Engine.MaterialInstanceDynamic)
  (Rendering|Material|SetScalarParameterValue material "TotalFilas" totalFilas :!class /Script/Engine.MaterialInstanceDynamic)
  (Rendering|Material|SetScalarParameterValue material "columna" columna :!class /Script/Engine.MaterialInstanceDynamic)
  (Rendering|Material|SetScalarParameterValue material "fila" fila :!class /Script/Engine.MaterialInstanceDynamic)
  (Rendering|Material|SetScalarParameterValue material "GradientWidthL" (.x _output_2) :!class /Script/Engine.MaterialInstanceDynamic)
  (Rendering|Material|SetScalarParameterValue material "GradientSuavizadoL" (.y _output_2) :!class /Script/Engine.MaterialInstanceDynamic)
  (Rendering|Material|SetScalarParameterValue material "GradientWidthR" (.x _output_3) :!class /Script/Engine.MaterialInstanceDynamic)
  (Rendering|Material|SetScalarParameterValue material "GradientSuavizadoR" (.y _output_3) :!class /Script/Engine.MaterialInstanceDynamic)
  (Rendering|Material|SetScalarParameterValue material "GradientWidthT" (.x _output_4) :!class /Script/Engine.MaterialInstanceDynamic)
  (Rendering|Material|SetScalarParameterValue material "GradientSuavizadoT" (.y _output_4) :!class /Script/Engine.MaterialInstanceDynamic)
  (Rendering|Material|SetScalarParameterValue material "GradientWidthB" (.x _output) :!class /Script/Engine.MaterialInstanceDynamic)
  (Rendering|Material|SetScalarParameterValue material "GradientSuavizadoB" (.y _output) :!class /Script/Engine.MaterialInstanceDynamic)
  (Rendering|Material|SetScalarParameterValue material "hue" (Utilities|Array|Get(acopy) HSB) :!class /Script/Engine.MaterialInstanceDynamic)
  (Rendering|Material|SetScalarParameterValue material "saturacion" (Utilities|Array|Get(acopy) HSB 1) :!class /Script/Engine.MaterialInstanceDynamic)
  (Rendering|Material|SetScalarParameterValue material "brillo" (Utilities|Array|Get(acopy) HSB 2) :!class /Script/Engine.MaterialInstanceDynamic)
  (return))