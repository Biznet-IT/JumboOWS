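; Game instance for a multi-instance screen-warping app that persists warp calibration and handles LAN session setup.
; Grid, edge gradients, HSB, camera and point settings are written to a MiSaveGame, with slots keyed by the MiPlayerController's PlayerIndex for saving, loading and resetting.
; FindSesionAndJoin joins the first LAN session found, or creates one and opens MapWarping as a listen server, flagging the instance as client or server.
; Network errors are only printed on screen.
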(event Custom|SaveConfigWarp
  (bind _returnvalue (Game|GetPlayerController 0))
  (bind _asmi_player_controller (Utilities|Casting|CastToMiPlayerController _returnvalue))
  (bind _playerindex (Variables|/Game/BP/MotionMx/blueprints/MiPlayerController.MiPlayerController_C|GetplayerIndex _asmi_player_controller))
  ;[0 0 0] Save Warp config to disk
  (SaveGame|SaveGametoSlot (Variables|Default|GetGameSave) (Utilities|String|Append (Variables|Default|GetGameSaveSlot) (Utilities|String|ToString(Integer) _playerindex)))
  (Development|PrintString (Utilities|String|Append "salvando configuracion para instancia -> " (Utilities|String|ToString(Integer) _playerindex)) true true "(R=0.000000,G=0.660000,B=1.000000,A=1.000000)" 1e+01))

(event Custom|FindSesionAndJoin
  ;[0.03646 0.03646 0.03646] find session and join
  ;[0 0 0] este metodo se tarda unos segundos en responder
  (bind _results (|FindSessions (Game|GetPlayerController 0) 3 true)
    (:OnSuccess
      (if (> (Utilities|Array|Length _results) 0)
        ;[0 0 0] Join founded SERVER
        (Development|PrintString "SERVER ENCONTRADO, CONECTANDO..." true true "(R=0.000000,G=0.367140,B=1.000000,A=1.000000)" 4.0)
        (bind _output_get (Variables|Default|SetServerFound (Utilities|Array|Get(acopy) _results)))
        (Development|PrintString (Class|FindSessionsCallbackProxy|GetServerName _output_get) true true "(R=0.000000,G=1.000000,B=0.207987,A=1.000000)" 5.0)
        (|JoinSession (Game|GetPlayerController 0) (Variables|Default|GetServerFound) ; Joins and auto loads the server map in this client
          (:OnSuccess
            (Development|PrintString "JOIN SUCCESS" true true "(R=0.000000,G=1.000000,B=0.116213,A=1.000000)" 4.0)
            (Variables|Default|SetInstanceIsClient true))
          (:OnFailure
            (Development|PrintString "JOIN ERROR" true true "(R=1.000000,G=0.000000,B=0.030547,A=1.000000)" 4.0)))
        (else
          ;[0 0 0] Create NEW SERVER
          (Development|PrintString "CREANDO SERVER" true true "(R=0.985164,G=1.000000,B=0.000000,A=1.000000)" 4.0)
          (|Session (Game|GetPlayerController 0) 100 true
            (:OnSuccess
              (Development|PrintString "SERVER CREADO" true true "(R=0.000000,G=1.000000,B=0.116213,A=1.000000)" 4.0)
              (Variables|Default|SetInstanceIsServer true)
              (Game|OpenLevel(byName) "MapWarping" true "listen"))
            (:OnFailure
              (Development|PrintString "CREACION DE SEVER FALLO !" true true "(R=1.000000,G=0.000000,B=0.030547,A=1.000000)" 4.0))))))
    (:OnFailure
      (Development|PrintString "NO SERVIDOR,  posiblemente hubo un problema de red" true true "(R=1.000000,G=0.000000,B=0.009844,A=1.000000)"))))

(event Custom|UpdateSaveGameValuesAndSave
  (params (GridW :type Integer) (GridH :type Integer) (GridRows :type Integer) (GridCols :type Integer) (Gradients :type Array%20of%20Vector%202D%20Structures) (HSB :type Array%20of%20Floats%20%28double-precision%29) (CamLocation :type Vector) (CamRotation :type Rotator) (puntos :type Array%20of%20Vectors) (FOV :type Float%20%28double-precision%29))
  ;[0 0.007042 0.03646] Save Values to Save Object
  (Utilities|FlowControl|Sequence
    (:then_0
      (Variables|/Game/BP/MotionMx/blueprints/MiSaveGame.MiSaveGame_C|SetGridSize (Variables|Default|GetGameSave) (Math|Vector2D|MakeVector2D (Math|Conversions|ToFloat(Integer) GridW) (Math|Conversions|ToFloat(Integer) GridH))))
    (:then_1
      (Variables|/Game/BP/MotionMx/blueprints/MiSaveGame.MiSaveGame_C|SetGridRows (Variables|Default|GetGameSave) GridRows))
    (:then_2
      (Variables|/Game/BP/MotionMx/blueprints/MiSaveGame.MiSaveGame_C|SetGridCols (Variables|Default|GetGameSave) GridCols))
    (:then_3
      (Variables|/Game/BP/MotionMx/blueprints/MiSaveGame.MiSaveGame_C|SetGradients (Variables|Default|GetGameSave) (Utilities|Map|MakeMap "Left" (Utilities|Array|Get(acopy) Gradients) "Right" (Utilities|Array|Get(acopy) Gradients 1) "Top" (Utilities|Array|Get(acopy) Gradients 2) "Bottom" (Utilities|Array|Get(acopy) Gradients 3))))
    (:then_4
      (Variables|/Game/BP/MotionMx/blueprints/MiSaveGame.MiSaveGame_C|SetHSB (Variables|Default|GetGameSave) (Utilities|Map|MakeMap "hue" (Utilities|Array|Get(acopy) HSB) "desaturacion" (Utilities|Array|Get(acopy) HSB 1) "brillo" (Utilities|Array|Get(acopy) HSB 2))))
    (:then_5
      (Variables|/Game/BP/MotionMx/blueprints/MiSaveGame.MiSaveGame_C|SetCamTransform (Variables|Default|GetGameSave) (Math|Transform|MakeTransform CamLocation CamRotation)))
    (:then_6
      (Variables|/Game/BP/MotionMx/blueprints/MiSaveGame.MiSaveGame_C|SetPoints (Variables|Default|GetGameSave) puntos))
    (:then_7
      (Variables|/Game/BP/MotionMx/blueprints/MiSaveGame.MiSaveGame_C|SetCamFOV (Variables|Default|GetGameSave) FOV))
    (:then_8
      (CallFunction|SaveConfigWarp))))

(event Custom|ResetSavedGameObject
  ;[0 0 0] reset saved warp config
  (SaveGame|DeleteGameinSlot (Utilities|String|Append (Variables|Default|GetGameSaveSlot) (Utilities|String|ToString(Integer) (Variables|/Game/BP/MotionMx/blueprints/MiPlayerController.MiPlayerController_C|GetplayerIndex (.AsMi%20Player%20Controller (Utilities|Casting|CastToMiPlayerController (Game|GetPlayerController 0)))))))
  (bind _returnvalue (SaveGame|CreateSaveGameObject "/Game/BP/MotionMx/blueprints/MiSaveGame.MiSaveGame_C"))
  (Variables|Default|SetGameSave _returnvalue)
  (CallFunction|SaveConfigWarp))

(event Custom|LoadOrCreateStoreObject
  (bind _returnvalue (Game|GetPlayerController 0))
  (bind _asmi_player_controller (Utilities|Casting|CastToMiPlayerController _returnvalue))
  (bind _playerindex (Variables|/Game/BP/MotionMx/blueprints/MiPlayerController.MiPlayerController_C|GetplayerIndex _asmi_player_controller))
  (bind _returnvalue_2 (Utilities|String|ToString(Integer) _playerindex))
  (Development|PrintString (Utilities|String|Append "cargando configuracion para instancia ->" _returnvalue_2))
  ;[0 0 0] SAVE game object       load or create
  (bind _returnvalue_3 (SaveGame|LoadGamefromSlot (Utilities|String|Append (Variables|Default|GetGameSaveSlot) _returnvalue_2)))
  (bind _asmi_save_game (Utilities|Casting|CastToMiSaveGame _returnvalue_3)
    (:then
      (Variables|Default|SetGameSave _asmi_save_game))
    (:CastFailed
      (bind _returnvalue_4 (SaveGame|CreateSaveGameObject "/Game/BP/MotionMx/blueprints/MiSaveGame.MiSaveGame_C"))
      (Variables|Default|SetGameSave _returnvalue_4))))

(event EventHandleNetworkError
  (params (FailureType :type ENetworkFailure%20Enum :default "NetDriverAlreadyExists") (bIsServer :type Boolean))
  ;[0 0 0] Handle Nework Error
  (Development|PrintString "NETWORK ERROR  !!" true true "(R=1.000000,G=0.000000,B=0.026519,A=1.000000)" 5.0)
  (Development|PrintString (Utilities|String|EnumtoString FailureType) true true "(R=1.000000,G=0.000000,B=0.026519,A=1.000000)" 5.0)
  (switch Utilities|FlowControl|Switch|SwitchonENetworkFailure FailureType
    (:ConnectionLost
      (Development|PrintString "CONNECTION LOST  :S"))))

(event EventInit)