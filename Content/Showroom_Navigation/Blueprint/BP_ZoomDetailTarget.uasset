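; Clickable zoom hotspot for showroom navigation, with an icon button, optional text label and its own spring-arm camera.
; The construction script sets up camera angle, arm length and FOV (copied from BP_MasterPawn), and sizes the billboard, trigger box and label.
; Valid clicks or non-drag touches store this point's ZoomDetailPointArray index in the game instance, then call the Zoom01 dispatcher.
; When labels are on, Tick turns the pivot toward the player camera.
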(event OnInputTouchEnd(Box_Trigger)
  (params (FingerIndex :type ETouchIndex%20Enum :default "Touch1") (TouchedComponent :type Primitive%20Component%20Object%20Reference))
  ;[1 1 1] Do not open when Touch is moving
  (bind _asbp_gameinstance_showroom (Utilities|Casting|CastToBP_Gameinstance_showroom (Game|GetGameInstance)))
  (if (not (Variables|/Game/Showroom_Navigation/Gameinstance/BP_Gameinstance_showroom.BP_Gameinstance_showroom_C|Getis_Touch_moving _asbp_gameinstance_showroom))
    ;[1 1 1] Find_this ZoomPoint in Array
    (bind _asbp_gameinstance_showroom_2 (Utilities|Casting|CastToBP_Gameinstance_showroom (Game|GetGameInstance)))
    (Variables|/Game/Showroom_Navigation/Gameinstance/BP_Gameinstance_showroom.BP_Gameinstance_showroom_C|SetGI_GetZoom _asbp_gameinstance_showroom_2 (Utilities|Array|FindItem (Variables|/Game/Showroom_Navigation/Gameinstance/BP_Gameinstance_showroom.BP_Gameinstance_showroom_C|GetZoomDetailPoint_Array _asbp_gameinstance_showroom_2) self))
    (Default|CallEventDispatcherZoom01)))

(event OnClicked(Box_Trigger)
  (params (TouchedComponent :type Primitive%20Component%20Object%20Reference) (ButtonPressed :type Key%20Structure))
  ;[1 1 1] Do not open when Touch is moving
  (bind _asbp_gameinstance_showroom (Utilities|Casting|CastToBP_Gameinstance_showroom (Game|GetGameInstance)))
  (if (not (Variables|/Game/Showroom_Navigation/Gameinstance/BP_Gameinstance_showroom.BP_Gameinstance_showroom_C|Getis%20first%20touch _asbp_gameinstance_showroom))
    ;[1 1 1] Find_this ZoomPoint in Array
    (bind _asbp_gameinstance_showroom_2 (Utilities|Casting|CastToBP_Gameinstance_showroom (Game|GetGameInstance)))
    (Variables|/Game/Showroom_Navigation/Gameinstance/BP_Gameinstance_showroom.BP_Gameinstance_showroom_C|SetGI_GetZoom _asbp_gameinstance_showroom_2 (Utilities|Array|FindItem (Variables|/Game/Showroom_Navigation/Gameinstance/BP_Gameinstance_showroom.BP_Gameinstance_showroom_C|GetZoomDetailPoint_Array _asbp_gameinstance_showroom_2) self))
    (Default|CallEventDispatcherZoom01)))

(event EventBeginPlay
  ;[1 1 1] enable click
  (bind _asplayer_controller (Utilities|Casting|CastToPlayerController (Game|GetPlayerController 0)))
  (Variables|/Script/Engine.PlayerController|SetbEnableClickEvents _asplayer_controller true))

(event EventTick
  (params (DeltaSeconds :type Float%20%28single-precision%29))
  ;[1 1 1] Text_Labels
  (if (Variables|Default|GetTextLabelsOn)
    (Transformation|SetWorldRotation (Variables|Default|GetPivot) (Math|Rotator|FindLookatRotation (Transformation|GetActorLocation) (Transformation|GetActorLocation (Game|GetPlayerCameraManager 0))) false false)))

(fn ConstructionScript
  (bind _button_size (Variables|Default|GetButton_Size))
  (bind _textrender (Variables|Default|GetTextRender))
  (bind _text_size (Variables|Default|GetText_Size))
  (bind _textonlysize (Variables|Default|GetTextOnlySize))
  (bind _returnvalue (/ _button_size 32.0))
  ;[1 1 1] Show Textlabels?
  (if (Variables|Default|GetTextLabelsOn)
    (Rendering|SetVisibility _textrender true false)
    (else
      (Rendering|SetVisibility _textrender false false)))
  ;[1 1 1] Set Camera
  (Transformation|SetRelativeRotation (Variables|Default|GetSpringArm) (Variables|Default|GetCamera%20Rotation) false false)
  (Variables|/Script/Engine.SpringArmComponent|SetTargetArmLength (Variables|Default|GetSpringArm) (Variables|Default|GetZoom%20Detail%20Point%2001%20Armlength))
  ;[1 1 1] Set FOV from Pawn
  (bind _returnvalue_2 (Actor|GetActorOfClass "/Game/Showroom_Navigation/Blueprint/BP_MasterPawn.BP_MasterPawn_C"))
  (Camera|SetFieldOfView (Variables|Default|GetCamera) (Variables|/Game/Showroom_Navigation/Blueprint/BP_MasterPawn.BP_MasterPawn_C|GetField_of_View _returnvalue_2))
  ;[1 1 1] Button Offset
  (Transformation|SetRelativeLocation (Variables|Default|GetIcon_group) (Variables|Default|GetButton_Offset) false false)
  ;[1 1 1] root lock rotation
  (Transformation|SetWorldRotation (Variables|Default|GetDefaultSceneRoot1) "0, 0, 0" false false)
  ;[1 1 1] Set Billboard
  (Class|MaterialBillboardComponent|SetElements (Variables|Default|GetMaterialBillboard) (Utilities|Array|MakeArray (Utilities|Struct|MakeMaterialSpriteElement (Variables|Default|GetBillboard) 0 false _button_size _button_size)))
  ;[1 1 1] Set Text
  (Rendering|Components|TextRender|SetText (Variables|Default|GetTextRender) (Utilities|Text|ToText(String) (Variables|Default|GetText%20Label)))
  ;[1 1 1] Set Box collider size to Button
  (Transformation|SetRelativeScale3D (Variables|Default|GetBox_Trigger) (Math|Vector|MakeVector _returnvalue _returnvalue _returnvalue))
  ;[1 1 1] Text Size and offset
  (Transformation|SetRelativeScale3D _text_size (Math|Vector|MakeVector (.x _textonlysize) (.y _textonlysize) (.z _textonlysize)))
  (Transformation|SetRelativeLocation _text_size (Math|Vector|MakeVector 0.0 (Variables|Default|GetText_Offset) 0.0) false false))

(fn TourButtonLabels
  (return ""))