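; Showroom game state that switches the player between BP_MasterPawn with WBP_Main and first-person walkthrough mode.
; BeginPlay restores the mode and first-person transform saved in the Game Instance, while WBP_Main's dispatcher triggers later switches to first person.
; First-person entry swaps widgets, toggles tagged actor arrays through nested loops and adds a joystick for touch.
; The first-person widget's Home and Back events are relayed through bridge dispatchers.
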(event Custom|CustomEvent
  ;[1 1 1] Button Home
  (Default|CallEventDispatcherHomeandResetBridge))

(event Custom|FP_Event_0
  ;[1 1 1] Posses Master Pawn
  (CallFunction|FPShow/HideTagObjectsFunction)
  ;[1 1 1] Posses_FP_character
  (bind _asbp_gameinstance_showroom (Utilities|Casting|CastToBP_Gameinstance_showroom (Game|GetGameInstance)))
  (Pawn|UnPossess (Game|GetPlayerController 0))
  (bind _returnvalue (Actor|GetActorOfClass "/Game/Showroom_Navigation/Blueprint/FirstPerson/BP_FirstPersonCharacter.BP_FirstPersonCharacter_C"))
  (Pawn|Possess (Game|GetPlayerController 0) _returnvalue)
  ;[1 1 1] Set_FP_Widget
  (Viewport|RemoveAllWidgets)
  (bind _returnvalue_2 (UserInterface|CreateWidget "/Game/Showroom_Navigation/Blueprint/UI_Widget/WBP_First_Person_Free.WBP_First_Person_Free_C" (Game|GetPlayerController 0)))
  (UserInterface|Viewport|AddtoViewport _returnvalue_2 0)
  (if (Math|Boolean|ORBoolean (Variables|/Game/Showroom_Navigation/Gameinstance/BP_Gameinstance_showroom.BP_Gameinstance_showroom_C|GetGI_Level%203%20On/off _asbp_gameinstance_showroom) (Variables|/Game/Showroom_Navigation/Gameinstance/BP_Gameinstance_showroom.BP_Gameinstance_showroom_C|GetGI_Level%202%20On/off _asbp_gameinstance_showroom) (Variables|/Game/Showroom_Navigation/Gameinstance/BP_Gameinstance_showroom.BP_Gameinstance_showroom_C|Getis%20Waypoint _asbp_gameinstance_showroom))
    ;[1 1 1] Set FP Position to camera Position
    (bind _asbp_gameinstance_showroom_2 (Utilities|Casting|CastToBP_Gameinstance_showroom (Game|GetGameInstance)))
    (bind _returnvalue_3 (Actor|GetActorOfClass "/Game/Showroom_Navigation/Blueprint/FirstPerson/BP_FirstPersonCharacter.BP_FirstPersonCharacter_C"))
    (Transformation|SetActorLocation _returnvalue_3 (Variables|/Game/Showroom_Navigation/Gameinstance/BP_Gameinstance_showroom.BP_Gameinstance_showroom_C|GetGI_DefaultSceneRoot_LevelSwitch _asbp_gameinstance_showroom_2) false false)
    (Pawn|SetControlRotation (Game|GetPlayerController 0) (Variables|/Game/Showroom_Navigation/Gameinstance/BP_Gameinstance_showroom.BP_Gameinstance_showroom_C|GetGI_ArmRotation_LevelSwitch _asbp_gameinstance_showroom_2))
    (else
      ;[1 1 1] Set FP -Actor - on self Position in Level 1
      (bind _returnvalue_4 (Actor|GetActorOfClass "/Game/Showroom_Navigation/Blueprint/FirstPerson/BP_FirstPersonCharacter.BP_FirstPersonCharacter_C"))
      (Transformation|SetActorLocation _returnvalue_4 (Transformation|GetActorLocation _returnvalue) false false)))
  ;[1 1 1] Set input Mode
  (Input|SetInputModeGameandUI (Game|GetPlayerController 0) 0 "DoNotLock" true false)
  ;[1 1 1] Set FP on
  (bind _asbp_gameinstance_showroom_3 (Utilities|Casting|CastToBP_Gameinstance_showroom (Game|GetGameInstance)))
  (Variables|/Game/Showroom_Navigation/Gameinstance/BP_Gameinstance_showroom.BP_Gameinstance_showroom_C|SetFPS_ON _asbp_gameinstance_showroom_3 true)
  ;[1 1 1] If Touch make Joystick
  (if (Variables|/Game/Showroom_Navigation/Gameinstance/BP_Gameinstance_showroom.BP_Gameinstance_showroom_C|Getis%20first%20touch _asbp_gameinstance_showroom_3)
    (Class|PlayerController|ActivateTouchInterface (Game|GetPlayerController 0) "/Game/Showroom_Navigation/MobileResources/HUD/LeftVirtualJoystickOnly.LeftVirtualJoystickOnly"))
  (Utilities|FlowControl|Sequence
    (:then_0
      ;[1 1 1] Button Home
      (bind _foundwidgets (Widget|GetAllWidgetsOfClass "/Game/Showroom_Navigation/Blueprint/UI_Widget/WBP_First_Person_Free.WBP_First_Person_Free_C" true))
      (EventDispatchers|BindEventtoHomeandResetEventDispatcher _foundwidgets (delegate Custom|Home_and_reset)))
    (:then_1
      ;[1 1 1] Button Back
      (bind _foundwidgets_2 (Widget|GetAllWidgetsOfClass "/Game/Showroom_Navigation/Blueprint/UI_Widget/WBP_First_Person_Free.WBP_First_Person_Free_C" true))
      (EventDispatchers|BindEventtoEventDispatcherBacktoPawn _foundwidgets_2 (delegate Custom|Back_to_pawn)))))

(event Custom|Home_and_reset
  ;[1 1 1] Button Home
  (Default|CallEventDispatcherHomeandResetBridge))

(event Custom|CustomEvent_1
  ;[1 1 1] Button Back
  (Default|CallEventDispatchterBacktoPawnBridge))

(event Custom|Back_to_pawn
  ;[1 1 1] Button Back
  (Default|CallEventDispatchterBacktoPawnBridge))

(event EventBeginPlay
  (bind _returnvalue (Game|GetPlayerController 0))
  ;[1 1 1] Is FPS ON?
  (bind _asbp_gameinstance_showroom (Utilities|Casting|CastToBP_Gameinstance_showroom (Game|GetGameInstance)))
  (if (Variables|/Game/Showroom_Navigation/Gameinstance/BP_Gameinstance_showroom.BP_Gameinstance_showroom_C|GetFPS_ON _asbp_gameinstance_showroom)
    (CallFunction|FPShow/HideTagObjectsFunction)
    ;[1 1 1] Posses FP Actor
    (Pawn|UnPossess _returnvalue)
    (bind _returnvalue_2 (Actor|GetActorOfClass "/Game/Showroom_Navigation/Blueprint/FirstPerson/BP_FirstPersonCharacter.BP_FirstPersonCharacter_C"))
    (Pawn|Possess _returnvalue _returnvalue_2)
    ;[1 1 1] Create FP Widget
    (Viewport|RemoveAllWidgets)
    (Utilities|FlowControl|Delay 0.2)
    (bind _returnvalue_3 (UserInterface|CreateWidget "/Game/Showroom_Navigation/Blueprint/UI_Widget/WBP_First_Person_Free.WBP_First_Person_Free_C" (Game|GetPlayerController 0)))
    (UserInterface|Viewport|AddtoViewport _returnvalue_3 0)
    ;[1 1 1] Set Lamera Position
    (bind _asbp_gameinstance_showroom_2 (Utilities|Casting|CastToBP_Gameinstance_showroom (Game|GetGameInstance)))
    (bind _returnvalue_4 (Actor|GetActorOfClass "/Game/Showroom_Navigation/Blueprint/FirstPerson/BP_FirstPersonCharacter.BP_FirstPersonCharacter_C"))
    (Pawn|SetControlRotation (Game|GetPlayerController 0) (Variables|/Game/Showroom_Navigation/Gameinstance/BP_Gameinstance_showroom.BP_Gameinstance_showroom_C|Getcontroler_rotation _asbp_gameinstance_showroom_2))
    (Transformation|SetActorTransform _returnvalue_4 (Variables|/Game/Showroom_Navigation/Gameinstance/BP_Gameinstance_showroom.BP_Gameinstance_showroom_C|GetPlayertransform _asbp_gameinstance_showroom_2))
    ;[1 1 1] set input Mode
    (Input|SetInputModeGameandUI (Game|GetPlayerController 0) 0 "DoNotLock" true false)
    ;[1 1 1] Is Touch make Joystick
    (bind _asbp_gameinstance_showroom_3 (Utilities|Casting|CastToBP_Gameinstance_showroom (Game|GetGameInstance)))
    (if (Variables|/Game/Showroom_Navigation/Gameinstance/BP_Gameinstance_showroom.BP_Gameinstance_showroom_C|Getis%20first%20touch _asbp_gameinstance_showroom_3)
      (Class|PlayerController|ActivateTouchInterface (Game|GetPlayerController 0) "/Game/Showroom_Navigation/MobileResources/HUD/LeftVirtualJoystickOnly.LeftVirtualJoystickOnly"))
    (Utilities|FlowControl|Sequence
      (:then_0
        ;[1 1 1] Button Home
        (bind _foundwidgets (Widget|GetAllWidgetsOfClass "/Game/Showroom_Navigation/Blueprint/UI_Widget/WBP_First_Person_Free.WBP_First_Person_Free_C" true))
        (EventDispatchers|BindEventtoHomeandResetEventDispatcher _foundwidgets (delegate Custom|CustomEvent)))
      (:then_1
        ;[1 1 1] Button Back
        (bind _foundwidgets_2 (Widget|GetAllWidgetsOfClass "/Game/Showroom_Navigation/Blueprint/UI_Widget/WBP_First_Person_Free.WBP_First_Person_Free_C" true))
        (EventDispatchers|BindEventtoEventDispatcherBacktoPawn _foundwidgets_2 (delegate Custom|CustomEvent_1))))
    (else
      ;[1 1 1] Posses Master Pawn
      (Viewport|RemoveAllWidgets)
      (bind _returnvalue_5 (Actor|GetActorOfClass "/Game/Showroom_Navigation/Blueprint/BP_MasterPawn.BP_MasterPawn_C"))
      (Pawn|Possess (Game|GetPlayerController 0) _returnvalue_5)
      (bind _returnvalue_6 (UserInterface|CreateWidget "/Game/Showroom_Navigation/Blueprint/UI_Widget/WBP_Main.WBP_Main_C"))
      (UserInterface|Viewport|AddtoViewport _returnvalue_6 0)
      (Widget|SetIsEnabled (Variables|/Game/Showroom_Navigation/Blueprint/UI_Widget/WBP_Main.WBP_Main_C|GetBack_Button _returnvalue_6) false)
      (Utilities|FlowControl|Delay 0.2)
      (Widget|SetIsEnabled (Variables|/Game/Showroom_Navigation/Blueprint/UI_Widget/WBP_Main.WBP_Main_C|GetBack_Button _returnvalue_6) true)
      (bind _foundwidgets_3 (Widget|GetAllWidgetsOfClass "/Game/Showroom_Navigation/Blueprint/UI_Widget/WBP_Main.WBP_Main_C" false))
      (EventDispatchers|BindEventtoNewEventDispatcherFP _foundwidgets_3 (delegate Custom|FP_Event_0)))))

(fn ConstructionScript)

(fn FPShow/HideTagObjectsFunction
  ;[1 1 1] Read FP Actor Tags
  (bind _asbp_gameinstance_showroom (Utilities|Casting|CastToBP_Gameinstance_showroom (Game|GetGameInstance)))
  (for _array_element (Variables|/Game/Showroom_Navigation/Gameinstance/BP_Gameinstance_showroom.BP_Gameinstance_showroom_C|GetGI_Array_Level1_Actors _asbp_gameinstance_showroom)
    (Rendering|SetActorHiddenInGame _array_element true)
    (Collision|SetActorEnableCollision _array_element false)
    (for _array_element_2 (Variables|/Game/Showroom_Navigation/Gameinstance/BP_Gameinstance_showroom.BP_Gameinstance_showroom_C|GetGI_Array_Level2_Actors _asbp_gameinstance_showroom)
      (Rendering|SetActorHiddenInGame _array_element_2 true)
      (Collision|SetActorEnableCollision _array_element_2 false)
      (for _array_element_3 (Variables|/Game/Showroom_Navigation/Gameinstance/BP_Gameinstance_showroom.BP_Gameinstance_showroom_C|GetGI_Array_Level3_Actors _asbp_gameinstance_showroom)
        (Rendering|SetActorHiddenInGame _array_element_3 true)
        (Collision|SetActorEnableCollision _array_element_3 false)
        (for _array_element_4 (Variables|/Game/Showroom_Navigation/Gameinstance/BP_Gameinstance_showroom.BP_Gameinstance_showroom_C|GetGI_Array_FP_Actors _asbp_gameinstance_showroom)
          (Rendering|SetActorHiddenInGame _array_element_4 false)
          (Collision|SetActorEnableCollision _array_element_4 true))))))