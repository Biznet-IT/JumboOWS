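; BP_SaveGame is the save game object for the Inventory3D system, holding inventory, storage and equipment slots, money, storage initialization state and pending local storage items.
; Its Save event copies the passed-in data into its own variables, then writes itself to a single hardcoded slot.
; DeleteSave and DoesSaveGameExist remove and check that same slot.
; The file contains no loading logic.
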(event Custom|Save
  (params (Inventory%20Slots :type Map%20of%20E_ItemType%20Enums%20to%20Structs :default "NewEnumerator0") (Storage%20Slots :type Map%20of%20Strings%20to%20Structs) (Money :type Integer) (InitializedStorage? :type Map%20of%20Strings%20to%20Booleans) (Equipment%20Slots :type Map%20of%20E_EquipmentType%20Enums%20to%20Structs :default "NewEnumerator0") (Local%20Storage%20Items%20To%20Add :type Map%20of%20Strings%20to%20Structs))
  (Variables|Default|SetInventory%20Slots Inventory%20Slots)
  (Variables|Default|SetStorage%20Slots Storage%20Slots)
  (Variables|Default|SetMoney Money)
  (Variables|Default|SetInitialized%20Storage? InitializedStorage?)
  (Variables|Default|SetEquipment%20Slots Equipment%20Slots)
  (Variables|Default|SetLocal%20Storage%20Items%20To%20Add Local%20Storage%20Items%20To%20Add)
  (SaveGame|SaveGametoSlot self "1"))

(event Custom|Delete%20Save
  (SaveGame|DeleteGameinSlot "1"))

(fn DoesSaveGameExist
  (bind _returnvalue (SaveGame|DoesSaveGameExist "1"))
  (return _returnvalue))