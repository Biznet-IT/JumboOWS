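; BP_InteractionVolume is a box volume for interacting with inventory items, with an Interact function that serves as a template.
; Construction sizes the box from BoxExtent and removes the preset Widget when ShowWidget is off.
; Show/HideWidget creates or destroys a widget component; a looping timer removes it once the player exceeds the interaction distance from DT_InventorySettings.
; Interact just returns true, with unconnected example nodes showing item checks, consumption and slot return.
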(event Custom|CustomEvent_0
  (bind _widget_component (Variables|Default|GetWidget%20Component))
  ;[1 0.01518 0] Show/Hide Widget
  (bind _returnvalue (Utilities|GetDataTableRow "/Game/Inventory3D/DataTables/DT_InventorySettings.DT_InventorySettings" "Default_Settings")
    (:then
      (if (> (Math|Vector|VectorLength (- (Transformation|GetActorLocation (Game|GetPlayerCharacter 0)) (Transformation|GetActorLocation))) (.DistanceToInteractWithInteractionVolumeObjecttypemustbeWorldDynamic (Utilities|Struct|BreakS_BaseSettings (.BaseSettings (Utilities|Struct|BreakS_InventorySettings _returnvalue)))))
        (Utilities|IsValid _widget_component
          (:Is%20Valid
            (Components|DestroyComponent _widget_component)
            (Utilities|Time|ClearandInvalidateTimerbyHandle (Variables|Default|GetTimer))))))))

(event EventShow/HideWidget
  (params (Show? :type Boolean))
  ;[1 0.01518 0] Show/Hide Widget
  (if Show?
    (Utilities|IsValid (Variables|Default|GetWidget%20Component)
      (:Is%20Valid
        (Components|DestroyComponent (Variables|Default|GetWidget%20Component)))
      (:Is%20Not%20Valid
        _))
    (bind _returnvalue (AddComponent|AddWidgetComponent false))
    (Variables|Default|SetWidget%20Component _returnvalue)
    (bind _returnvalue_2 (Utilities|Time|SetTimerbyEvent (delegate Custom|CustomEvent_0) 3.0 true))
    (Variables|Default|SetTimer _returnvalue_2)
    (else
      (Utilities|IsValid (Variables|Default|GetWidget%20Component)
        (:Is%20Valid
          (Components|DestroyComponent (Variables|Default|GetWidget%20Component))
          (Utilities|Time|ClearandInvalidateTimerbyHandle (Variables|Default|GetTimer)))))))

(fn ConstructionScript
  (Components|Box|SetBoxExtent (Variables|Default|GetBox) (Variables|Default|GetBox%20Extent) false)
  (if (not (Variables|Default|GetShow%20Widget?))
    (Components|DestroyComponent (Variables|Default|GetWidget))))

(fn Interact
  (params (Item :type BP%20Master%20Item%20Object%20Reference) (Amount :type Integer) (Inventory :type BP%20Inventory%20Object%20Reference))
  (return true))