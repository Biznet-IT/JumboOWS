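; BP_PickUp_item is a world pickup for an inventory item, taking its mesh, scale and name from the ItemClass defaults.
; A widget component shows name and amount, toggled by focus.
; Interact adds the item to the given inventory, posts a HUD pickup notice and refreshes the label.
; The actor destroys itself when everything fits, otherwise it keeps the leftover amount.
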(event EventActorinFocuse
  (params (InFocuse :type Boolean))
  (bind _namewidget (Variables|Components|GetNameWidget))
  ;[0.3594 0 1] Hide / Show Item Name When Focuse
  (if InFocuse
    (Rendering|SetVisibility _namewidget true false)
    (else
      (Rendering|SetVisibility _namewidget false false))))

(event EventBeginPlay
  ;[1 0.4775 0] Get Widget Reference
  (bind _asitem_name_wb (Utilities|Casting|CastToItemNameWB (UserInterface|GetWidget (Variables|Components|GetNameWidget))))
  (Variables|Default|SetAs%20Item%20Name%20WB _asitem_name_wb)
  ;[0 0.9829 1] Set Widget Name And Amount
  (CallFunction|SetWidgetNameandAmount))

(fn ConstructionScript
  (bind _item_class (Variables|Default|GetItem%20Class))
  (bind _scale (Variables|Default|GetScale))
  (bind _item_structure (Utilities|GetClassDefaults _item_class))
  (bind (_name _description _3dmeshoneitem _3dmeshestwoandmoreitemsinstack _id _stackable _maxstack _usable _itemtype _weight _parameters _price _slottype _equipementtypes _pickupitemscale) (Utilities|Struct|BreakS_ItemData _item_structure))
  (bind _returnvalue (+ _pickupitemscale -1.0))
  (bind _returnvalue_2 (+ _scale _returnvalue))
  (Transformation|SetRelativeScale3D (Variables|Components|GetStaticMesh) (Math|Vector|MakeVector _returnvalue_2 _returnvalue_2 _returnvalue_2))
  (Components|StaticMesh|SetStaticMesh (Variables|Components|GetStaticMesh) _3dmeshoneitem))

(fn SetNameWidgetVisibility
  (params (bNewVisibility :type Boolean))
  (Rendering|SetVisibility (Variables|Components|GetNameWidget) bNewVisibility false)
  (return))

(fn PickUpItem
  (params (InventoryRef :type BP%20Inventory%20Object%20Reference))
  (bind (_all_items_added _items_added) (Default|AddItem InventoryRef (Variables|Default|GetItem%20Class) (Variables|Default|GetAmount) false false))
  (LocalVariables|SetLocal%20Items%20Added _items_added)
  (if _all_items_added
    (Actor|DestroyActor)
    (return (LocalVariables|GetLocal%20Items%20Added))
    (else
      (Variables|Default|SetAmount (- (Variables|Default|GetAmount) (LocalVariables|GetLocal%20Items%20Added)))
      (return (LocalVariables|GetLocal%20Items%20Added)))))

(fn SetWidgetNameandAmount
  (Default|SetText (Variables|Default|GetAs%20Item%20Name%20WB) (.Name (Utilities|Struct|BreakS_ItemData (.Item_Structure (Utilities|GetClassDefaults (Variables|Default|GetItem%20Class))))) (Variables|Default|GetAmount))
  (return))

(fn Interact
  (params (Inventory%20Ref :type BP%20Inventory%20Object%20Reference))
  (bind _items_added (CallFunction|PickUpItem Inventory%20Ref))
  (Default|AddPickUpWidgettoVerticalBox (Variables|/Game/Inventory3D/Inventory/Blueprints/Inventory/BP_Inventory.BP_Inventory_C|GetHUD%20Ref Inventory%20Ref) (.Name (Utilities|Struct|BreakS_ItemData (.Item_Structure (Utilities|GetClassDefaults (Variables|Default|GetItem%20Class))))) _items_added)
  ;[0 0.9829 1] Set Amount in Widget
  (CallFunction|SetWidgetNameandAmount)
  (return false))