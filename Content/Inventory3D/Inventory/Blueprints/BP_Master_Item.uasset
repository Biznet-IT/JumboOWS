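; Base actor for items in the 3D inventory, supporting drag and drop, rotation, stack splitting, discarding and use.
; Click raises the mesh and enables Tick, which follows the cursor and traces down from a point chosen by slot size and rotation to highlight slots.
; Release passes the traced slot to the inventory, which also handles stack changes.
; The mesh varies with stack amount, and a widget shows price.
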(event EventBeginPlay
  (Variables|Other|SetPlayer%20Controller (Game|GetPlayerController 0))
  ;[0 1 0.4375] Save The Relative Location Of Item
  (Variables|Other|SetRelative%20Location (Variables|/Script/Engine.SceneComponent|GetRelativeLocation (Variables|Components|GetStaticMesh)))
  ;[0.6359 1 0] Get Price Widget Ref
  (|GetPriceWidgetRef)
  ;[0.03125 0 1] Bug fix when Item not stackble but has more than one maximum stack parameter
  (|BugfixwhenItemnotstackblebuthasmorethanonemaximumstackparameter)
  ;[1 0.08557 0] Load Settings
  (bind _returnvalue (Utilities|GetDataTableRow "/Game/Inventory3D/DataTables/DT_InventorySettings.DT_InventorySettings" "Default_Settings")
    (:then
      (Variables|Other|SetRaising%20Item%20when%20pressed (.RaisingItemWhenPressed (Utilities|Struct|BreakS_BaseSettings (.basesettings _returnvalue)))))))

(event EventRotate
  ;[0 1 0.9531] Click Events
  ;;[0.7109 1 0] Rotate Item
  (CallFunction|RotateItem))

(event EventTick
  (params (DeltaSeconds :type Float%20%28single-precision%29))
  ;[1 0 0.04213] Tick Only Works When Actor Is Dragged
  ;[1 0.5156 0] Set Location When Draged
  (|SetLocation)
  ;[0.9453 1 0] Line Trace For Slot Detection
  (|LineTrace)
  ;[1 0 0.5859] Activate Slots Highlighting
  (Default|CallOnActiveteSlotHighLighting (Variables|Other|GetHit%20Actor) self (Utilities|GetClass self) (Variables|Other|GetInventory%20Slots)))

(event EventOnRelease
  (bind (_hitactor _hitcomponent) (CallFunction|CenterOfItemTrace))
  ;[0 1 0.9531] Click Events
  ;;[0.8984 0 1] On Release
  (Default|UnbindonActivateSlotHighlighting (Variables|Other|GetInventory%20Ref) self)
  ;;;[1 0 0.4688] Disable Actor Tick
  (Actor|Tick|SetActorTickEnabled false)
  ;;;[0 0.6719 1] Set Relative Location When Release
  (Transformation|SetRelativeLocation (Variables|Components|GetStaticMesh) (|Location) false false)
  ;;;[0 0.3672 1] Drag And Drop Operation
  (Default|DragandDrop (Variables|Other|GetInventory%20Ref) (Variables|Other|GetHit%20Actor) self (Variables|Other|GetInventory%20Slots) (Variables|Default|GetHit%20Component) (Variables|Other|GetIs%20item%20placed%20in%20storage) _hitcomponent _hitactor))

(event EventOnInventoryClose
  ;[1 0.9609 0] On closing inventory while dragging an item
  (Default|UnbindonActivateSlotHighlighting (Variables|Other|GetInventory%20Ref) self)
  (Actor|Tick|SetActorTickEnabled false)
  (Default|ReturnItemtoOwnSlot (Variables|Other|GetInventory%20Ref) self)
  (Transformation|SetActorRelativeLocation self (Variables|Other|GetRelative%20Location)))

(event EventUpdateItem
  (params (Amount :type Integer))
  ;[0.9453 1 0] Update Item Mesh On Changed Amount
  (CallFunction|ChangeStaticMesh Amount))

(event EventRemoveAll
  ;[0.875 1 0] Throw Away All Items In Slot
  (Default|ThrowAwayAllItemsinSlot (Variables|Other|GetInventory%20Ref) self))

(event EventOnClick
  ;[0 1 0.9531] Click Events
  ;;[1 0.4922 0] On Click
  (Default|AssignonActivateSlotHighlighting (Variables|Other|GetInventory%20Ref) self)
  ;;;[1 0.1855 0] Remove Item In Craft Place
  (if (Utilities|Enum|Equal(Enum) (Variables|/Game/Inventory3D/Inventory/Blueprints/Inventory/BP_Inventory.BP_Inventory_C|GetInventory%20Status (Variables|Other|GetInventory%20Ref)) "NewEnumerator4")
    (if (Default|FindIteminCraftPlace (Variables|Other|GetInventory%20Ref) self)
      (Default|ClearCraftItem (Variables|Other|GetInventory%20Ref) self)
      (else
        (Variables|Other|SetChached%20Rotation (Variables|Other|GetRotation) :!label _label)))
    (else
      (goto _label)))
  ;;;[0 1 0.7422] Enable Actor Tick
  (Actor|Tick|SetActorTickEnabled true)
  ;;;[0.1484 1 0] Set Relative Location When Clicked
  (Transformation|SetRelativeLocation (Variables|Components|GetStaticMesh) (+ (Variables|Other|GetRelative%20Location) (Math|Vector|MakeVector 0.0 0.0 (Variables|Other|GetRaising%20Item%20when%20pressed))) false false)
  (Default|OnClickEvent (Variables|Other|GetInventory%20Ref) (.ItemType (Utilities|Struct|BreakS_ItemData (Variables|Default|GetItem_Structure)))))

(event EventSplit
  (bind _self self)
  (bind _inventory_ref (Variables|Other|GetInventory%20Ref))
  (bind _amount (Default|GetItemAmountbyRef _inventory_ref _self))
  ;[0.0336 1 0] Split Item
  (if (!= _amount 2)
    (bind _returnvalue (UserInterface|CreateWidget "/Game/Inventory3D/Widgets/SplitConfirmWB.SplitConfirmWB_C" 0 (- _amount 1) (Variables|Other|GetInventory%20Ref) self))
    (UserInterface|Viewport|AddtoViewport _returnvalue 0)
    (else
      (Default|SplitItem (Variables|Other|GetInventory%20Ref) self 1))))

(event EventUseItem
  ;[1 0.4219 0] Use Item
  ;;[1 0.9141 0] Check the item is usable
  (if (Utilities|Enum|NotEqual(Enum) (.Usable (Utilities|Struct|BreakS_ItemData (.Item_Structure (Utilities|GetClassDefaults (Utilities|GetClass self))))) "NewEnumerator0")
    (Default|SubtractfromItembyRef (Variables|Other|GetInventory%20Ref) self 1)
    (CallFunction|UseItemLogic)))

(fn ConstructionScript
  (CallFunction|ChangeStaticMesh (.MaxStack (Utilities|Struct|BreakS_ItemData (Variables|Default|GetItem_Structure)))))

(fn LineTrace
  (params (Start :type Vector))
  (bind (_outhit _returnvalue) (Collision|LineTraceForObjects Start (+ Start (* (Transformation|GetActorUpVector) -10)) (Utilities|Array|MakeArray "ObjectTypeQuery1") false 0 "None" true "(R=1.000000,G=0.000000,B=0.000000,A=1.000000)" "(R=0.000000,G=1.000000,B=0.000000,A=1.000000)" 1.0))
  (return _outhit _returnvalue))

(fn RotateItem
  (bind _item_structure (Variables|Default|GetItem_Structure))
  (bind _slottype (Utilities|Struct|BreakS_ItemData _item_structure))
  (if (not (Math|Boolean|ORBoolean (Utilities|Enum|Equal(Enum) _slottype "NewEnumerator0") (Utilities|Enum|Equal(Enum) _slottype "NewEnumerator2") (Utilities|Enum|Equal(Enum) _slottype "NewEnumerator6")))
    (switch Utilities|FlowControl|Switch|SwitchonE_ItemRotation (Variables|Other|GetRotation)
      (:NewEnumerator0
        (Variables|Other|SetRotation "NewEnumerator1"))
      (:NewEnumerator1
        (Variables|Other|SetRotation "NewEnumerator0")))
    (Transformation|SetActorRelativeRotation (Utilities|Select :Index (Variables|Other|GetRotation) :NewEnumerator0 "0, 0, 0" :NewEnumerator1 "0,90.000000, 0"))
    (return)
    (else
      (return))))

(fn SetNewMesh
  (params (NewMesh :type Static%20Mesh%20Object%20Reference))
  (Components|StaticMesh|SetStaticMesh (Variables|Components|GetStaticMesh) NewMesh)
  (return))

(fn ChangeStaticMesh
  (params (Amount :type Integer))
  (bind _returnvalue (- Amount 2))
  (bind _item_structure (Variables|Default|GetItem_Structure))
  (bind _item_structure_2 (Variables|Default|GetItem_Structure))
  (bind _3dmeshestwoandmoreitemsinstack (Utilities|Struct|BreakS_ItemData _item_structure))
  (bind _3dmeshestwoandmoreitemsinstack_2 (Utilities|Struct|BreakS_ItemData _item_structure_2))
  (bind _returnvalue_2 (Utilities|Array|LastIndex _3dmeshestwoandmoreitemsinstack_2))
  (bind _output (Utilities|Array|Get(acopy) _3dmeshestwoandmoreitemsinstack _returnvalue_2))
  (if (== Amount 1)
    _
    (elif (Utilities|Array|IsValidIndex _3dmeshestwoandmoreitemsinstack_2 _returnvalue)
      (CallFunction|SetNewMesh (Utilities|Array|Get(acopy) _3dmeshestwoandmoreitemsinstack_2 _returnvalue))
      (return)
      (elif (== (Utilities|Array|Length _3dmeshestwoandmoreitemsinstack_2) 0)
        _
        (else
          (Utilities|IsValid _output
            (:Is%20Valid
              (CallFunction|SetNewMesh _output)
              (return))
            (:Is%20Not%20Valid
              _))))))
  (CallFunction|SetNewMesh (.3DMeshOneItem (Utilities|Struct|BreakS_ItemData (Variables|Default|GetItem_Structure))))
  (return))

(fn AddItem
  (params (ItemClass :type BP%20Master%20Item%20Class%20Reference) (Amount :type Integer))
  (bind (_all_items_added _items_added) (Default|AddItem (Variables|Other|GetInventory%20Ref) ItemClass Amount (Variables|Other|GetIs%20item%20placed%20in%20storage) false))
  (if _all_items_added
    (return)
    (else
      (Default|DropItemtoWorld (Variables|Other|GetInventory%20Ref) ItemClass (- Amount _items_added))
      (return))))

(fn GetParameters
  (bind _item_structure (Variables|Default|GetItem_Structure))
  (bind (_paramenername _minparameter _maxparameter _parameter) (Utilities|Struct|BreakS_ParametersStructure (.parameters _item_structure)))
  (return _minparameter _maxparameter _parameter))

(fn SetPriceWidget
  (params (Value :type Integer) (Visibility :type Boolean))
  (Default|SetPrice (Variables|Other|GetAs%20Price%20WB) Value)
  (Rendering|SetVisibility (Variables|Default|GetPriceWidget) Visibility true)
  (Development|SetHiddeninGame (Variables|Default|GetPriceWidget) (not Visibility) true))

(fn CenterOfItemTrace
  (bind (_outhit _returnvalue) (CallFunction|LineTrace (Transformation|GetWorldLocation (Variables|Default|GetOneSlot))))
  (return (.HitActor (Collision|BreakHitResult _outhit)) (.HitComponent (Collision|BreakHitResult _outhit))))

(fn GetSlotData
  (return (.slotone (Variables|Other|GetInventory%20Slots)) (Variables|Other|GetIs%20item%20placed%20in%20storage) (Variables|Other|GetIsEquippedItem?) (Variables|Other|GetEquipment%20Slot%20Ref)))