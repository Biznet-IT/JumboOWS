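; A single slot actor for the 3D inventory, drawn as a scaled plane that can also act as a named equipment slot.
; Highlight events show active, occupied or deactivated states through custom materials or a color-driven dynamic material instance.
; The construction script previews the name widget, which BeginPlay destroys.
; InitializeEquipmentSlot applies equipment settings, reinitializes materials, removes directional components and adds a manually redrawn name widget.
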(event EventBeginPlay
  (bind _slot_size (Variables|EquipmentSlotSettings|GetSlot%20Size))
  (bind (_x _y) (Math|Vector2D|BreakVector2D _slot_size))
  (CallFunction|InitializeMaterials)
  (Components|DestroyComponent (Variables|Default|GetEquipment%20Slot%20Name%20Widget))
  ;[1 0 0.06906] Set Custom Scale
  (Transformation|SetRelativeScale3D (Variables|Default|GetPlane) (Math|Vector|MakeVector _x _y 1.0)))

(event EventActivateSlotHighlighting
  (params (isEmptySlot? :type Boolean))
  (bind _custommaterials (Variables|Default|GetCustomMaterials))
  (bind _dynamicmaterial (Variables|Default|GetDynamicMaterial))
  (bind _slotcolors (Variables|Default|GetSlotColors))
  (bind (_color _opacity _emissivecolor) (Utilities|Struct|BreakS_SlotColor (.activeslot _slotcolors)))
  (bind (_color_2 _opacity_2 _emissivecolor_2) (Utilities|Struct|BreakS_SlotColor (.occupiedslot _slotcolors)))
  ;[0 0.08594 1] Higlighting
  (if (.usecustommaterials _custommaterials)
    (if isEmptySlot?
      (Rendering|Material|SetMaterial (Variables|Default|GetPlane) 0 (.activeslot _custommaterials))
      (else
        (Rendering|Material|SetMaterial (Variables|Default|GetPlane) 0 (.occupiedslot _custommaterials))))
    (elif isEmptySlot?
      (Rendering|Material|SetVectorParameterValue _dynamicmaterial "Color" _color :!class /Script/Engine.MaterialInstanceDynamic)
      (Rendering|Material|SetScalarParameterValue _dynamicmaterial "Opacity" _opacity :!class /Script/Engine.MaterialInstanceDynamic)
      (Rendering|Material|SetScalarParameterValue _dynamicmaterial "Emissive Color" _emissivecolor :!class /Script/Engine.MaterialInstanceDynamic)
      (Rendering|Material|SetMaterial (Variables|Default|GetPlane) 0 _dynamicmaterial)
      (else
        (Rendering|Material|SetVectorParameterValue _dynamicmaterial "Color" _color_2 :!class /Script/Engine.MaterialInstanceDynamic)
        (Rendering|Material|SetScalarParameterValue _dynamicmaterial "Opacity" _opacity_2 :!class /Script/Engine.MaterialInstanceDynamic)
        (Rendering|Material|SetScalarParameterValue _dynamicmaterial "Emissive Color" _emissivecolor_2 :!class /Script/Engine.MaterialInstanceDynamic)
        (Rendering|Material|SetMaterial (Variables|Default|GetPlane) 0 _dynamicmaterial)))))

(event EventDeactivateSlotHighlighting
  (bind _custommaterials (Variables|Default|GetCustomMaterials))
  (bind _dynamicmaterial (Variables|Default|GetDynamicMaterial))
  (bind _slotcolors (Variables|Default|GetSlotColors))
  (bind (_color _opacity _emissivecolor) (Utilities|Struct|BreakS_SlotColor (.deactivatedslot _slotcolors)))
  ;[0 0.08594 1] Higlighting
  (if (.usecustommaterials _custommaterials)
    (Rendering|Material|SetMaterial (Variables|Default|GetPlane) 0 (.deactivatedslot _custommaterials))
    (else
      (Rendering|Material|SetVectorParameterValue _dynamicmaterial "Color" _color :!class /Script/Engine.MaterialInstanceDynamic)
      (Rendering|Material|SetScalarParameterValue _dynamicmaterial "Opacity" _opacity :!class /Script/Engine.MaterialInstanceDynamic)
      (Rendering|Material|SetScalarParameterValue _dynamicmaterial "Emissive Color" _emissivecolor :!class /Script/Engine.MaterialInstanceDynamic)
      (Rendering|Material|SetMaterial (Variables|Default|GetPlane) 0 _dynamicmaterial))))

(fn ConstructionScript
  (bind _name_transform (Variables|EquipmentSlotSettings|GetName%20Transform))
  (bind _slot_size (Variables|EquipmentSlotSettings|GetSlot%20Size))
  (bind (_x _y) (Math|Vector2D|BreakVector2D _slot_size))
  (bind (_roll _pitch _yaw) (Math|Rotator|BreakRotator (.rotation _name_transform)))
  (Transformation|SetRelativeScale3D (Variables|Default|GetPlane) (Math|Vector|MakeVector _x _y 1.0))
  ;[1 0.2591 0] Set Custom Transform Of Name Widget
  (Transformation|SetRelativeTransform (Variables|Default|GetEquipment%20Slot%20Name%20Widget) (Math|Transform|MakeTransform (.location _name_transform) (Math|Rotator|MakeRotator (+ _roll 1.8e+02) (+ _pitch 9e+01) (+ _yaw 9e+01)) (.scale _name_transform)) false false)
  ;[1 0.7096 0] Set Equipment Slot Name
  (bind _asequipment_slot_name_wb (Utilities|Casting|CastToEquipmentSlotNameWB (UserInterface|GetWidget (Variables|Default|GetEquipment%20Slot%20Name%20Widget))))
  (Default|SetName _asequipment_slot_name_wb (Variables|EquipmentSlotSettings|GetName)))

(fn InitializeMaterials
  (bind _custommaterials (Variables|Default|GetCustomMaterials))
  (if (.usecustommaterials _custommaterials)
    (Rendering|Material|SetMaterial (Variables|Default|GetPlane) 0 (.deactivatedslot _custommaterials))
    (return)
    (else
      (bind _returnvalue (Rendering|Material|CreateDynamicMaterialInstance "/Game/Inventory3D/FilesOfInventory/Materials/Material_Instances/MI_DynamicMaterial.MI_DynamicMaterial" "None" "Transient" :!class /Script/Engine.KismetMaterialLibrary))
      (Variables|Default|SetDynamicMaterial _returnvalue)
      (CallFunction|DeactivateSlotHighlighting)
      (return))))

(fn InitializeEquipmentSlot
  (params (EqipementType :type E_EquipmentType%20Enum :default "NewEnumerator3") (This%20is%20Equipment%20Slot :type Boolean) (Can%20place%20a%20stack%20of%20items%20if%20it%20is%20an%20equipment%20slot :type Boolean) (Rotation%20In%20Equipment%20Slot :type E_ItemRotation%20Enum :default "NewEnumerator0") (SlotColors :type S%20Slot%20Colors%20Structure) (CustomMaterials :type S%20Custom%20Materials%20Structure))
  (bind _name_transform (Variables|EquipmentSlotSettings|GetName%20Transform))
  (bind (_roll _pitch _yaw) (Math|Rotator|BreakRotator (.rotation _name_transform)))
  (Variables|Default|SetEquipmentType EqipementType)
  (Variables|Default|SetThis%20is%20Equipment%20Slot This%20is%20Equipment%20Slot)
  (Variables|Default|SetCan%20place%20a%20stack%20of%20items%20if%20it%20is%20an%20equipment%20slot Can%20place%20a%20stack%20of%20items%20if%20it%20is%20an%20equipment%20slot)
  (Variables|Default|SetRotation%20In%20Equipment%20Slot Rotation%20In%20Equipment%20Slot)
  (Variables|Default|SetSlotColors SlotColors)
  (Variables|Default|SetCustomMaterials CustomMaterials)
  (CallFunction|InitializeMaterials)
  (Components|DestroyComponent (Variables|Default|GetDown))
  (bind _returnvalue (UserInterface|CreateWidget "/Game/Inventory3D/Widgets/EquipmentSlotNameWB.EquipmentSlotNameWB_C" 0 (Variables|EquipmentSlotSettings|GetName)))
  (LocalVariables|SetLocal%20Widget _returnvalue)
  (bind _returnvalue_2 (AddComponent|AddWidgetComponent false (Math|Transform|MakeTransform (.location _name_transform) (Math|Rotator|MakeRotator (+ _roll 1.8e+02) (+ _pitch 9e+01) (+ _yaw 9e+01)) (.scale _name_transform))))
  (UserInterface|SetWidget _returnvalue_2 (LocalVariables|GetLocal%20Widget))
  (Class|WidgetComponent|SetDrawatDesiredSize _returnvalue_2 true)
  (Class|WidgetComponent|SetManuallyRedraw _returnvalue_2 true)
  (Class|WidgetComponent|SetWindowFocusable _returnvalue_2 false)
  (Collision|SetCollisionEnabled _returnvalue_2 "NoCollision")
  (Rendering|SetCastShadow _returnvalue_2 false)
  (return))

(fn GetReference
  (return self))