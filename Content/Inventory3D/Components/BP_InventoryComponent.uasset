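; Player inventory component that spawns a 3D BP_Inventory actor attached to the owner's camera, with mouse-driven widget interaction.
; Exposes input, show/hide, save and load functions, optionally freezing movement while the inventory is open.
; Interaction presets (first person, third person, top down) size a pickup box, polled by timer for focus and prompts.
; Interact reaches items, storage and crafting through box overlaps, camera traces or cursor hits.
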(event EventBeginPlay
  ;[1 0.1345 0] Get Camera Component
  (Variables|Components|SetCamera%20Component (Actor|GetComponentbyClass (Components|GetOwner) "/Script/Engine.CameraComponent"))
  ;[1 0.2695 0] Get Player Controller
  (Variables|References|SetPlayer%20Controller (Game|GetPlayerController 0))
  ;[0 0.1484 1] Get Hud Reference
  (|GetHudRef)
  ;[0.1986 0 1] Spawn Inventory In The World
  (bind _returnvalue (Game|SpawnActorfromClass "/Game/Inventory3D/Inventory/Blueprints/Inventory/BP_Inventory.BP_Inventory_C" (Math|Transform|MakeTransform "0, 0, 0" "0, 0, 0" "1.000000,1.000000,1.000000") "AlwaysSpawn" (Components|GetOwner) (Variables|References|GetHUD%20Ref) 0))
  (Variables|References|SetInventory%20Ref _returnvalue)
  ;[0.4495 1 0] Create New Scene Component To Attach
  (bind _returnvalue_2 (Game|AddComponentbyClass (Components|GetOwner) "/Script/Engine.SceneComponent" false (Math|Transform|MakeTransform "28.931576,-22.999887,8.722985" "0,-90.000000,-90.000000" "1.000000,1.000000,1.000000")))
  (bind _output_get (Variables|Components|SetComponent%20to%20Attach _returnvalue_2))
  (Transformation|AttachComponentToComponent _output_get (Variables|Components|GetCamera%20Component) "None" "KeepRelative" "KeepRelative" "KeepRelative" false)
  ;[0 0.754 1] Attach Inventory To Scene Component
  (Transformation|AttachComponentToComponent (Variables|References|GetInventory%20Ref) (Variables|Components|GetComponent%20to%20Attach) "None" "SnapToTarget" "KeepRelative" "KeepRelative" false)
  ;[1 0.5012 0] Add Widget Interaction Component
  (bind _returnvalue_3 (Game|AddComponentbyClass (Components|GetOwner) "/Script/UMG.WidgetInteractionComponent" true))
  (bind _output_get_2 (Variables|Components|SetWidget%20Interactions _returnvalue_3))
  (Variables|/Script/UMG.WidgetInteractionComponent|SetInteractionSource _output_get_2 "Mouse")
  (Transformation|AttachComponentToComponent (Variables|Components|GetWidget%20Interactions) (Variables|Components|GetComponent%20to%20Attach) "None" "KeepRelative" "KeepRelative" "KeepRelative" false)
  ;[1 0.1943 0] Get Movement Component
  (Pawn|GetMovementComponent)
  ;[1 0 0.05645] Initialize Interactions Presets
  (|InitializeInteractionsPresets))

(fn AttachInventorytoComponent
  (params (Custom%20Component :type Scene%20Component%20Object%20Reference))
  (Utilities|IsValid (Variables|Components|GetComponent%20to%20Attach)
    (:Is%20Valid
      (Components|DestroyComponent (Variables|Components|GetComponent%20to%20Attach)))
    (:Is%20Not%20Valid
      _))
  (Variables|Components|SetComponent%20to%20Attach Custom%20Component)
  (Transformation|AttachComponentToComponent (Variables|References|GetInventory%20Ref) (Variables|Components|GetComponent%20to%20Attach) "None" "SnapToTarget" "KeepRelative" "KeepRelative" false)
  (return))

(fn LeftPressed
  (params (Key :type Key%20Structure :default "None"))
  (Class|WidgetInteractionComponent|PressPointerKey (Variables|Components|GetWidget%20Interactions) Key)
  (Default|LeftClickEvents (Variables|References|GetInventory%20Ref) true)
  (return))

(fn LeftReleased
  (params (Key :type Key%20Structure :default "None"))
  (Class|WidgetInteractionComponent|ReleasePointerKey (Variables|Components|GetWidget%20Interactions) Key)
  (Default|LeftClickEvents (Variables|References|GetInventory%20Ref) false)
  (return))

(fn RightClick
  (Default|RightClickEvents (Variables|References|GetInventory%20Ref))
  (return))

(fn Show\HideInventory
  (bind _isvisible_ (Default|Show/HideInventory (Variables|References|GetInventory%20Ref)))
  (Variables|Other|SetIs%20Visible%20Inventory? _isvisible_)
  (Interactions|DisableMovement)
  (return (Variables|Other|GetIs%20Visible%20Inventory?)))

(fn Show\HideCraft
  (bind _isvisible_ (Default|Hide/ShowCtaft (Variables|References|GetInventory%20Ref)))
  (Variables|Other|SetIs%20Visible%20Inventory? _isvisible_)
  (Interactions|DisableMovement)
  (return (Variables|Other|GetIs%20Visible%20Inventory?)))

(fn Show\HideEquipmentSlots
  (params (Show%20Equipments%20Slots%20Only%20In%20This%20Tab :type Boolean) (Show%20Equipment%20Slots%20In%20All%20Tabs%20%28Override%29 :type Boolean) (Open%20This%20Tab%20When%20Opened :type Boolean) (Tab :type E_ItemType%20Enum :default "NewEnumerator0"))
  (bind _isvisible_ (Default|Show/HideEquipmentSlots (Variables|References|GetInventory%20Ref) Show%20Equipment%20Slots%20In%20All%20Tabs%20%28Override%29 Open%20This%20Tab%20When%20Opened Show%20Equipments%20Slots%20Only%20In%20This%20Tab Tab))
  (Variables|Other|SetIs%20Visible%20Inventory? _isvisible_)
  (Interactions|DisableMovement)
  (return (Variables|Other|GetIs%20Visible%20Inventory?)))

(fn RemoveSave
  (Default|DeleteSave (Variables|References|GetInventory%20Ref))
  (return))

(fn GetHudReference
  (return (Variables|References|GetHUD%20Ref)))

(fn GetInventoryReference
  (return (Variables|References|GetInventory%20Ref)))

(fn DisableMovement
  (if (Variables|Default|GetDisable%20Movement%20When%20Opened)
    (Variables|Default|GetMovement%20Component
      (:then
        (if (Variables|Other|GetIs%20Visible%20Inventory?)
          (if (Utilities|Enum|Equal(Enum) (Variables|/Script/Engine.CharacterMovementComponent|GetMovementMode (Variables|Default|GetMovement%20Component)) "MOVE_None")
            (return)
            (else
              (Variables|Other|SetMovement%20Mode (Variables|/Script/Engine.CharacterMovementComponent|GetMovementMode (Variables|Default|GetMovement%20Component)))
              (Pawn|Components|CharacterMovement|DisableMovement (Variables|Default|GetMovement%20Component))
              (return)))
          (else
            (Pawn|Components|CharacterMovement|SetMovementMode (Variables|Default|GetMovement%20Component) (Variables|Other|GetMovement%20Mode) 0)
            (return))))
      (:else
        (return)))
    (else
      (return))))

(fn Show\HideInteractionWidget
  (params (Show? :type Boolean))
  (if Show?
    (Default|Show\HideInteractWidget (Variables|References|GetHUD%20Ref) true)
    (return)
    (else
      (Default|Show\HideInteractWidget (Variables|References|GetHUD%20Ref) false)
      (return))))

(fn SetShowVisibleItemsNames
  (if (Utilities|Enum|Equal(Enum) (Variables|Default|GetInteraction%20Presets) "NewEnumerator2")
    (if (Variables|Other|GetIs%20Visible%20Inventory?)
      (Default|Show\HideInteractWidget (Variables|References|GetHUD%20Ref) false)
      (bind _hit_actor (Variables|Other|GetHit%20Actor)
        (:then
          (Class|BPCharacterActorsInteraction|ActorinFocuse(Message) _hit_actor false)
          (Variables|Other|SetHit%20Actor 0)
          (return))
        (:else
          (return)))
      (else
        (bind _hit_actor_2 (Variables|Other|GetHit%20Actor)
          (:then
            (Class|BPCharacterActorsInteraction|ActorinFocuse(Message) _hit_actor_2 false)
            (Variables|Other|SetHit%20Actor 0))
          (:else
            _))
        (LocalVariables|SetLocal%20Hit%20Actor (.HitActor (Collision|BreakHitResult (.HitResult (Game|Player|GetHitResultUnderCursorbyChannel (Variables|References|GetPlayer%20Controller) "TraceTypeQuery1" false)))))
        (for _array_element (Collision|GetOverlappingActors (Variables|Components|GetBox%20Collision) "/Script/Engine.Actor" :!class /Script/Engine.PrimitiveComponent)
          (if (== _array_element (LocalVariables|GetLocal%20Hit%20Actor))
            (Variables|Other|SetHit%20Actor (LocalVariables|GetLocal%20Hit%20Actor))
            (Utilities|IsValid (Utilities|Array|Get(acopy) (Class|Actor|GetComponentsbyInterface (LocalVariables|GetLocal%20Hit%20Actor) "/Game/Inventory3D/FilesOfInventory/Interfaces/BP_Character_Actors_Interaction.BP_Character_Actors_Interaction_C"))
              (:Is%20Valid
                (LocalVariables|SetLocal%20Is%20Interaction%20Object%20in%20Focus? true))
              (:Is%20Not%20Valid
                _))
            (Utilities|Array|RemoveItem (Variables|Other|GetItemsInFocuse) (LocalVariables|GetLocal%20Array%20Element))))
        (Interactions|Show\HideInteractionWidget (LocalVariables|GetLocal%20Is%20Interaction%20Object%20in%20Focus?))
        (bind _hit_actor_3 (Variables|Other|GetHit%20Actor)
          (:then
            (Class|BPCharacterActorsInteraction|ActorinFocuse(Message) _hit_actor_3 true)
            (return))
          (:else
            (return)))))
    (elif (Variables|Other|GetIs%20Visible%20Inventory?)
      (for _array_element_2 (Variables|Other|GetItemsInFocuse)
        (bind _output_get (LocalVariables|SetLocal%20Array%20Element _array_element_2))
        (Utilities|IsValid _output_get
          (:Is%20Valid
            (Class|BPCharacterActorsInteraction|ActorinFocuse(Message) (LocalVariables|GetLocal%20Array%20Element) false)
            (Utilities|Array|RemoveItem (Variables|Other|GetItemsInFocuse) (LocalVariables|GetLocal%20Array%20Element)))
          (:Is%20Not%20Valid
            (Utilities|Array|RemoveItem (Variables|Other|GetItemsInFocuse) (LocalVariables|GetLocal%20Array%20Element)))))
      (Default|Show\HideInteractWidget (Variables|References|GetHUD%20Ref) false)
      (return)
      (else
        (for _array_element_3 (Collision|GetOverlappingActors (Variables|Components|GetBox%20Collision) "/Script/Engine.Actor" :!class /Script/Engine.PrimitiveComponent)
          (LocalVariables|SetLocal%20Array%20Element _array_element_3)
          (Utilities|Array|AddUnique (Variables|Other|GetItemsInFocuse) (LocalVariables|GetLocal%20Array%20Element))
          (Class|BPCharacterActorsInteraction|ActorinFocuse(Message) (LocalVariables|GetLocal%20Array%20Element) true))
        (for _array_element_4 (Variables|Other|GetItemsInFocuse)
          (LocalVariables|SetLocal%20Array%20Element _array_element_4)
          (if (== (Utilities|Array|FindItem (Collision|GetOverlappingActors (Variables|Components|GetBox%20Collision) "/Game/Inventory3D/Inventory/Blueprints/BP_PickUp_item.BP_PickUp_item_C" :!class /Script/Engine.PrimitiveComponent) (LocalVariables|GetLocal%20Array%20Element)) -1)
            (Utilities|IsValid (LocalVariables|GetLocal%20Array%20Element)
              (:Is%20Valid
                (Class|BPCharacterActorsInteraction|ActorinFocuse(Message) (LocalVariables|GetLocal%20Array%20Element) false)
                (if (Utilities|Array|IsValidIndex (Class|Actor|GetComponentsbyInterface (LocalVariables|GetLocal%20Array%20Element) "/Game/Inventory3D/FilesOfInventory/Interfaces/BP_Character_Actors_Interaction.BP_Character_Actors_Interaction_C"))
                  (LocalVariables|SetLocal%20Is%20Interaction%20Object%20in%20Focus? true))
                (Utilities|Array|RemoveItem (Variables|Other|GetItemsInFocuse) (LocalVariables|GetLocal%20Array%20Element)))
              (:Is%20Not%20Valid
                (Utilities|Array|RemoveItem (Variables|Other|GetItemsInFocuse) (LocalVariables|GetLocal%20Array%20Element))))))
        (Interactions|Show\HideInteractionWidget (LocalVariables|GetLocal%20Is%20Interaction%20Object%20in%20Focus?))
        (return)))))

(fn Interact
  (bind _inventory_ref (Variables|References|GetInventory%20Ref))
  (bind _itemsinfocuse (Variables|Other|GetItemsInFocuse))
  (bind _camera_component (Variables|Components|GetCamera%20Component))
  (bind _returnvalue (Transformation|GetWorldLocation _camera_component))
  (bind _output (Utilities|Array|Get(acopy) _itemsinfocuse))
  (bind _inventory_status (Variables|/Game/Inventory3D/Inventory/Blueprints/Inventory/BP_Inventory.BP_Inventory_C|GetInventory%20Status _inventory_ref))
  (if (Utilities|Enum|Equal(Enum) "NewEnumerator1" (Variables|/Game/Inventory3D/Inventory/Blueprints/Inventory/BP_Inventory.BP_Inventory_C|GetInventory%20Status (Variables|References|GetInventory%20Ref)))
    (Utilities|FlowControl|Sequence
      (:then_0
        (Utilities|IsValid _output
          (:Is%20Valid
            (Class|BPCharacterActorsInteraction|Interact(Message) _output (Variables|References|GetInventory%20Ref))
            (Default|CallOnInteract (Variables|References|GetInventory%20Ref) "NewEnumerator0"))))
      (:then_1
        (switch Utilities|FlowControl|Switch|SwitchonE_InteractionPresets (Variables|Default|GetInteraction%20Presets)
          (:NewEnumerator3
            (bind (_outhit _returnvalue_2) (Collision|LineTraceByChannel _returnvalue (+ _returnvalue (* (Math|Vector|GetForwardVector _camera_component) 5e+02)) "TraceTypeQuery1" false 0 "None" :!label _label))
            (if _returnvalue_2
              (Utilities|IsValid (Actor|GetComponentbyClass (.HitActor (Collision|BreakHitResult _outhit)) "/Game/Inventory3D/Components/BP_StorageAndStoreComponents.BP_StorageAndStoreComponents_C")
                (:Is%20Valid
                  (bind _return (Class|BPCharacterActorsInteraction|Interact(Message) (Actor|GetComponentbyClass (.HitActor (Collision|BreakHitResult _outhit)) "/Game/Inventory3D/Components/BP_StorageAndStoreComponents.BP_StorageAndStoreComponents_C") (Variables|References|GetInventory%20Ref)))
                  (Variables|Other|SetIs%20Visible%20Inventory? _return)
                  (Interactions|DisableMovement)
                  (return))
                (:Is%20Not%20Valid
                  (Utilities|IsValid (Actor|GetComponentbyClass (.HitActor (Collision|BreakHitResult _outhit)) "/Game/Inventory3D/Components/BP_Craft_Component.BP_Craft_Component_C")
                    (:Is%20Valid
                      (bind _return_2 (Class|BPCharacterActorsInteraction|Interact(Message) (Actor|GetComponentbyClass (.HitActor (Collision|BreakHitResult _outhit)) "/Game/Inventory3D/Components/BP_Craft_Component.BP_Craft_Component_C") (Variables|References|GetInventory%20Ref)))
                      (Variables|Other|SetIs%20Visible%20Inventory? _return_2)
                      (Interactions|DisableMovement)
                      (Default|CallOnInteract (Variables|References|GetInventory%20Ref) "NewEnumerator2")
                      (return))
                    (:Is%20Not%20Valid
                      (return)))))
              (else
                (return))))
          (:NewEnumerator0
            (goto _label))
          (:NewEnumerator1
            (if (Variables|Other|GetIs%20Visible%20Inventory?)
              (return)
              (else
                (for _array_element (Collision|GetOverlappingActors (Variables|Components|GetBox%20Collision) "/Script/Engine.Actor" :!class /Script/Engine.PrimitiveComponent)
                  (Utilities|IsValid _array_element
                    (:Is%20Valid
                      (for _array_element_2 (Class|Actor|GetComponentsbyInterface _array_element "/Game/Inventory3D/FilesOfInventory/Interfaces/BP_Character_Actors_Interaction.BP_Character_Actors_Interaction_C")
                        (Utilities|IsValid _array_element_2
                          (:Is%20Valid
                            (bind _return_3 (Class|BPCharacterActorsInteraction|Interact(Message) _array_element_2 (Variables|References|GetInventory%20Ref)))
                            (Variables|Other|SetIs%20Visible%20Inventory? _return_3)
                            (Interactions|DisableMovement)
                            (if (and (Variables|Other|GetIs%20Visible%20Inventory?) (Components|ComponentHasTag _array_element_2 "CraftComponent"))
                              (Default|CallOnInteract (Variables|References|GetInventory%20Ref) "NewEnumerator2"))))))))
                (return))))
          (:NewEnumerator2
            (if (Variables|Other|GetIs%20Visible%20Inventory?)
              (return)
              (else
                (LocalVariables|SetLocal%20Hit%20Actor (.HitActor (Collision|BreakHitResult (.HitResult (Game|Player|GetHitResultUnderCursorbyChannel (Variables|References|GetPlayer%20Controller) "TraceTypeQuery1" true)))))
                (bind _array_element_3 (Utilities|Array|ForEachLoopwithBreak (Collision|GetOverlappingActors (Variables|Components|GetBox%20Collision) "/Script/Engine.Actor" :!class /Script/Engine.PrimitiveComponent) :!label _label_2)
                  (:LoopBody
                    (if (== (LocalVariables|GetLocal%20Hit%20Actor) _array_element_3)
                      (bind _return_4 (Class|BPCharacterActorsInteraction|Interact(Message) (LocalVariables|GetLocal%20Hit%20Actor) (Variables|References|GetInventory%20Ref)))
                      (Variables|Other|SetIs%20Visible%20Inventory? _return_4)
                      (Interactions|DisableMovement)
                      (Default|CallOnInteract (Variables|References|GetInventory%20Ref) "NewEnumerator0")
                      (bind _local_hit_actor (LocalVariables|GetLocal%20Hit%20Actor)
                        (:then
                          (for _array_element_4 (Class|Actor|GetComponentsbyInterface _local_hit_actor "/Game/Inventory3D/FilesOfInventory/Interfaces/BP_Character_Actors_Interaction.BP_Character_Actors_Interaction_C")
                            (bind _return_5 (Class|BPCharacterActorsInteraction|Interact(Message) _array_element_4 (Variables|References|GetInventory%20Ref)))
                            (Variables|Other|SetIs%20Visible%20Inventory? _return_5)
                            (Interactions|DisableMovement)
                            (goto _label_2 Break)))
                        (:else
                          (goto _label_2 Break)))))
                  (:Completed
                    (return)))))))))
    (elif (Math|Boolean|ORBoolean (Utilities|Enum|Equal(Enum) "NewEnumerator4" _inventory_status) (Utilities|Enum|Equal(Enum) "NewEnumerator3" _inventory_status) (Utilities|Enum|Equal(Enum) "NewEnumerator2" _inventory_status))
      (Input|Show\HideInventory)
      (return)
      (else
        (return)))))

(fn InventoryIsVisible?
  (return (select (Utilities|Enum|Equal(Enum) (Variables|Default|GetInteraction%20Presets) "NewEnumerator3") (Variables|/Game/Inventory3D/Inventory/Blueprints/Inventory/BP_Inventory.BP_Inventory_C|GetInventory%20Is%20Visible? (Variables|References|GetInventory%20Ref)) (Variables|Other|GetIs%20Visible%20Inventory?))))

(fn VisualizePickUpBoxCollision
  (bind _returnvalue (Components|GetOwner))
  (bind _length (Variables|InteractCollisionOptions|GetLength))
  (bind _returnvalue_2 (Actor|GetComponentbyClass _returnvalue "/Script/Engine.CapsuleComponent"))
  (Variables|Components|SetCamera%20Component (Actor|GetComponentbyClass (Components|GetOwner) "/Script/Engine.CameraComponent"))
  (bind _returnvalue_3 (Game|AddComponentbyClass (Components|GetOwner) "/Script/Engine.BoxComponent" false))
  (bind _output_get (Variables|Components|SetBox%20Collision _returnvalue_3))
  (Transformation|AttachComponentToComponent _output_get (Utilities|Select :Index (Variables|Default|GetInteraction%20Presets) :NewEnumerator3 _returnvalue_2 :NewEnumerator0 (Variables|Components|GetCamera%20Component) :NewEnumerator1 _returnvalue_2 :NewEnumerator2 _returnvalue_2) "None" "SnapToTarget" "KeepRelative" "SnapToTarget" false)
  (Transformation|SetRelativeLocation (Variables|Components|GetBox%20Collision) (Math|Vector|MakeVector (Utilities|Select :Index (Variables|Default|GetInteraction%20Presets) :NewEnumerator3 0.0 :NewEnumerator0 _length :NewEnumerator1 _length :NewEnumerator2 0.0) 0.0 0.0) false false)
  (Components|Box|SetBoxExtent (Variables|Components|GetBox%20Collision) (Math|Vector|MakeVector (Variables|InteractCollisionOptions|GetLength) (Variables|InteractCollisionOptions|GetWidth) (Variables|InteractCollisionOptions|GetHeight)) true)
  (return))

(fn AttachInventorytoCameraComponent
  (params (Parent :type Scene%20Component%20Object%20Reference))
  (Transformation|AttachComponentToComponent (Variables|Components|GetComponent%20to%20Attach) Parent "None" "KeepRelative" "KeepRelative" "KeepRelative" false)
  (return))

(fn Save
  (Default|Save (Variables|References|GetInventory%20Ref))
  (return))

(fn Load
  (if (Utilities|Enum|Equal(Enum) (Default|GetInventoryStatus (Variables|References|GetInventory%20Ref)) "NewEnumerator1")
    (bind _outactors (Actor|GetAllActorsOfClasswithTag "/Script/Engine.Actor" "Storage"))
    (for _array_element _outactors
      (Utilities|Array|Clear (Variables|/Game/Inventory3D/Components/BP_StorageAndStoreComponents.BP_StorageAndStoreComponents_C|GetItems%20To%20Add%20 (Actor|GetComponentbyClass _array_element "/Game/Inventory3D/Components/BP_StorageAndStoreComponents.BP_StorageAndStoreComponents_C")))
      (Variables|/Game/Inventory3D/Components/BP_StorageAndStoreComponents.BP_StorageAndStoreComponents_C|SetInitialized (Actor|GetComponentbyClass _array_element "/Game/Inventory3D/Components/BP_StorageAndStoreComponents.BP_StorageAndStoreComponents_C") false)
      (Variables|/Game/Inventory3D/Components/BP_StorageAndStoreComponents.BP_StorageAndStoreComponents_C|SetSlots%20Data (Actor|GetComponentbyClass _array_element "/Game/Inventory3D/Components/BP_StorageAndStoreComponents.BP_StorageAndStoreComponents_C") ""))
    (bind _outactors_2 (Actor|GetAllActorsOfClass "/Game/Inventory3D/Inventory/Blueprints/Inventory/BP_InventorySlot.BP_InventorySlot_C"))
    (for _array_element_2 _outactors_2
      (Actor|DestroyActor _array_element_2))
    (bind _outactors_3 (Actor|GetAllActorsOfClass "/Game/Inventory3D/Inventory/Blueprints/BP_Master_Item.BP_Master_Item_C"))
    (for _array_element_3 _outactors_3
      (Actor|DestroyActor _array_element_3))
    (Actor|DestroyActor (Variables|References|GetInventory%20Ref))
    (bind _returnvalue (Game|SpawnActorfromClass "/Game/Inventory3D/Inventory/Blueprints/Inventory/BP_Inventory.BP_Inventory_C" (Math|Transform|MakeTransform "0, 0, 0" "0, 0, 0" "1.000000,1.000000,1.000000") "AlwaysSpawn" (Components|GetOwner) (Variables|References|GetHUD%20Ref) 0))
    (Variables|References|SetInventory%20Ref _returnvalue)
    (Transformation|AttachComponentToComponent (Variables|References|GetInventory%20Ref) (Variables|Components|GetComponent%20to%20Attach) "None" "SnapToTarget" "KeepRelative" "KeepRelative" false)
    (Variables|Other|SetIs%20Visible%20Inventory? false)
    (Variables|/Script/Engine.PlayerController|SetbShowMouseCursor (Variables|References|GetPlayer%20Controller) false)
    (Input|SetInputModeGameOnly (Variables|References|GetPlayer%20Controller) false)
    (Interactions|DisableMovement)
    (return)
    (else
      (return))))

(fn TakeAllItemsinStorage
  (Default|TakeAllItemsinStorage (Variables|References|GetInventory%20Ref))
  (return))

(fn CustomInteraction
  (params (Interact%20with :type Actor%20Object%20Reference))
  (bind _return (Class|BPCharacterActorsInteraction|Interact(Message) Interact%20with (Variables|References|GetInventory%20Ref)))
  (if _return
    (return true)
    (else
      (for _array_element (Class|Actor|GetComponentsbyInterface Interact%20with "/Game/Inventory3D/FilesOfInventory/Interfaces/BP_Character_Actors_Interaction.BP_Character_Actors_Interaction_C")
        (bind _return_2 (Class|BPCharacterActorsInteraction|Interact(Message) _array_element (Variables|References|GetInventory%20Ref)))
        (LocalVariables|SetLocal%20Interact? _return_2))
      (return (LocalVariables|GetLocal%20Interact?)))))

(fn CustomFocusonItem
  (params (Interact%20with :type Actor%20Object%20Reference) (InFocuse? :type Boolean))
  (Class|BPCharacterActorsInteraction|ActorinFocuse(Message) Interact%20with InFocuse?)
  (for _array_element (Class|Actor|GetComponentsbyInterface Interact%20with "/Game/Inventory3D/FilesOfInventory/Interfaces/BP_Character_Actors_Interaction.BP_Character_Actors_Interaction_C")
    (Class|BPCharacterActorsInteraction|ActorinFocuse(Message) _array_element InFocuse?))
  (return))