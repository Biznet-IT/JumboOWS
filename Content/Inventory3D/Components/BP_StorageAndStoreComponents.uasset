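; Actor component that turns its owner into a storage container or store for the 3D inventory, tagging it "Storage" on BeginPlay.
; Interact passes its grid, layout, mesh and saved slot settings to the inventory, seeds preset items until initialized, and toggles price display for stores.
; Items added through AddItemInStorageStore queue until the next Interact.
; SaveSlots records slot contents, item rotations and occupied indexes for later reopening.
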(event Custom|Add%20Items
  (params (Target :type BP%20Inventory%20Object%20Reference))
  ;[0 0.4391 1] Add Items From "AddItems" Variable On First Initialize
  (CallFunction|AddItemsonInitialize (Variables|Default|GetAddItems) Target))

(event EventBeginPlay
  ;[1 0.8144 0] Add "Storage" tag to owner for easier searching
  (Utilities|Array|Add (Variables|/Script/Engine.Actor|GetTags (Components|GetOwner)) "Storage"))

(fn SaveSlots
  (params (Array :type Array%20of%20BP%20Inventory%20Slot%20Object%20References))
  (Variables|Default|SetSlots%20Data "")
  (for _array_element Array
    (Utilities|Array|Add (.slotsdata (Variables|Default|GetSlots%20Data)) (Variables|/Game/Inventory3D/Inventory/Blueprints/Inventory/BP_InventorySlot.BP_InventorySlot_C|GetSlot_Structure _array_element))
    (Utilities|Array|Add (.rotation (Variables|Default|GetSlots%20Data)) (select (and (.NotEmpty (Utilities|Struct|BreakS_InventorySlot (Variables|/Game/Inventory3D/Inventory/Blueprints/Inventory/BP_InventorySlot.BP_InventorySlot_C|GetSlot_Structure _array_element))) (not (.ItisPartOfItem (Utilities|Struct|BreakS_InventorySlot (Variables|/Game/Inventory3D/Inventory/Blueprints/Inventory/BP_InventorySlot.BP_InventorySlot_C|GetSlot_Structure _array_element))))) (Variables|/Game/Inventory3D/Inventory/Blueprints/BP_Master_Item.BP_Master_Item_C|GetRotation (.ItemObject (Utilities|Struct|BreakS_InventorySlot (Variables|/Game/Inventory3D/Inventory/Blueprints/Inventory/BP_InventorySlot.BP_InventorySlot_C|GetSlot_Structure _array_element)))) "NewEnumerator0"))
    (Utilities|Array|Add (.slotindexes (Variables|Default|GetSlots%20Data)) (select (and (.NotEmpty (Utilities|Struct|BreakS_InventorySlot (Variables|/Game/Inventory3D/Inventory/Blueprints/Inventory/BP_InventorySlot.BP_InventorySlot_C|GetSlot_Structure _array_element))) (not (.ItisPartOfItem (Utilities|Struct|BreakS_InventorySlot (Variables|/Game/Inventory3D/Inventory/Blueprints/Inventory/BP_InventorySlot.BP_InventorySlot_C|GetSlot_Structure _array_element))))) (Variables|/Game/Inventory3D/Inventory/Blueprints/BP_Master_Item.BP_Master_Item_C|GetInventory%20Slots (.ItemObject (Utilities|Struct|BreakS_InventorySlot (Variables|/Game/Inventory3D/Inventory/Blueprints/Inventory/BP_InventorySlot.BP_InventorySlot_C|GetSlot_Structure _array_element)))) "")))
  (return))

(fn InteractwithStorage
  (params (Inventory :type BP%20Inventory%20Object%20Reference))
  (bind _initialized (Default|InitializeStorage\Store Inventory (Variables|Default|GetSlots%20Per%20Row) (Variables|Default|GetSlots%20Per%20Colum) self (Variables|Default|GetSlots%20Data) (Variables|Default|GetDenny%20Item%20Type) (Variables|Default|GetThis%20is%20Store) (Variables|Transform|GetSet%20Slots%20Scale) (Variables|Transform|GetOffset%20to%20the%20Right) (Variables|Transform|GetOffset%20to%20the%20Down) (Variables|Transform|GetOffset%20to%20the%20Forward) (Variables|Transform|GetRotation) (Variables|Transform|GetCustom%20Transform) (Variables|Transform|GetUse%20Custom%20Transform) (Variables|StaticMesh|GetInitialize%20Mesh) (Variables|StaticMesh|GetStatic%20Mesh) (Variables|StaticMesh|GetStatic%20Mesh%20Transform)))
  (if (Variables|Default|GetInitialized)
    _
    (else
      (Variables|Default|SetInitialized _initialized)
      (CallFunction|AddItems Inventory)))
  (Default|SetVisibilityOfPriceWidget Inventory (Variables|Default|GetThis%20is%20Store))
  (return _initialized))

(fn AddIteminStorage\Store
  (params (Item :type BP%20Master%20Item%20Class%20Reference) (Amaunt :type Integer))
  (Utilities|Array|Add (Variables|Default|GetItems%20To%20Add%20) (Utilities|Struct|MakeS_CraftItems Item Amaunt))
  (return))

(fn AddItemsonInitialize
  (params (Array :type Array%20of%20S%20Craft%20Items%20Structures) (Inventory%20Ref :type BP%20Inventory%20Object%20Reference))
  (for _array_element Array
    (if (Utilities|IsValidClass (.item _array_element))
      (Default|AddItem Inventory%20Ref (.item _array_element) (.amaunt _array_element) true false)))
  (return))

(fn Interact
  (params (Inventory%20Ref :type BP%20Inventory%20Object%20Reference))
  (bind _initialized (Default|InitializeStorage\Store Inventory%20Ref (Variables|Default|GetSlots%20Per%20Row) (Variables|Default|GetSlots%20Per%20Colum) self (Variables|Default|GetSlots%20Data) (Variables|Default|GetDenny%20Item%20Type) (Variables|Default|GetThis%20is%20Store) (Variables|Transform|GetSet%20Slots%20Scale) (Variables|Transform|GetOffset%20to%20the%20Right) (Variables|Transform|GetOffset%20to%20the%20Down) (Variables|Transform|GetOffset%20to%20the%20Forward) (Variables|Transform|GetRotation) (Variables|Transform|GetCustom%20Transform) (Variables|Transform|GetUse%20Custom%20Transform) (Variables|StaticMesh|GetInitialize%20Mesh) (Variables|StaticMesh|GetStatic%20Mesh) (Variables|StaticMesh|GetStatic%20Mesh%20Transform) (Variables|Transform|GetSize%20Of%20Slot)))
  (if (Variables|Default|GetInitialized)
    _
    (else
      (Variables|Default|SetInitialized _initialized)
      (CallFunction|AddItems Inventory%20Ref)))
  (Default|SetVisibilityOfPriceWidget Inventory%20Ref (Variables|Default|GetThis%20is%20Store))
  (CallFunction|AddItemsonInitialize (Variables|Default|GetItems%20To%20Add%20) Inventory%20Ref)
  (Utilities|Array|Clear (Variables|Default|GetItems%20To%20Add%20))
  (return _initialized))