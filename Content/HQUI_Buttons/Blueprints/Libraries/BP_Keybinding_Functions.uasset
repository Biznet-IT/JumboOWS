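; Blueprint function library for querying and rebinding action and axis input mappings through Input Settings for keybinding buttons.
; Lookups find whether a key is bound, its mapping name, and the gamepad or keyboard/mouse key for a name.
; Rebinds replace the same-device binding, clear another mapping holding the new key, then rebuild and save keymaps.
; Thumbstick helpers classify stick directions and can convert them to X/Y axis keys.
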(fn DoesKeybindingExist
  (params (Key :type Key%20Structure))
  (if (.ReturnValue (Utility|DoesKeyExistinActionMapping Key))
    (return true)
    (elif (.ReturnValue (Utility|DoesKeyExistinAxisMapping Key))
      (return true)
      (else
        (return false)))))

(fn DoesKeyExistinActionMapping
  (params (Key :type Key%20Structure))
  (bind _returnvalue (Class|InputSettings|GetInputSettings))
  (bind _actionnames (Class|InputSettings|GetActionNames _returnvalue))
  (if (Utilities|Array|IsValidIndex _actionnames)
    (bind _array_element (Utilities|Array|ForEachLoopwithBreak _actionnames)
      (:LoopBody
        (bind _array_element_2 (Utilities|Array|ForEachLoopwithBreak (Class|InputSettings|GetActionMappingbyName (Class|InputSettings|GetInputSettings) _array_element) :!label _label)
          (:LoopBody
            (if (== (.Key (Utilities|Struct|BreakInputActionKeyMapping _array_element_2)) Key)
              (LocalVariables|SetbFound true)
              (LocalVariables|SetKeyMapping _array_element_2)
              (goto _label Break)))))
      (:Completed
        (return (LocalVariables|GetbFound) (LocalVariables|GetKeyMapping))))
    (else
      (return (LocalVariables|GetbFound) (LocalVariables|GetKeyMapping)))))

(fn DoesKeyExistinAxisMapping
  (params (Key :type Key%20Structure))
  (bind _returnvalue (Class|InputSettings|GetInputSettings))
  (bind _axisnames (Class|InputSettings|GetAxisNames _returnvalue))
  (if (Utilities|Array|IsValidIndex _axisnames)
    (bind _array_element (Utilities|Array|ForEachLoopwithBreak _axisnames)
      (:LoopBody
        (bind _array_element_2 (Utilities|Array|ForEachLoopwithBreak (Class|InputSettings|GetAxisMappingbyName (Class|InputSettings|GetInputSettings) _array_element) :!label _label)
          (:LoopBody
            (if (== (.Key (Utilities|Struct|BreakInputAxisKeyMapping _array_element_2)) Key)
              (LocalVariables|SetbFound true)
              (LocalVariables|SetKeyMapping _array_element_2)
              (goto _label Break)))))
      (:Completed
        (return (LocalVariables|GetbFound) (LocalVariables|GetKeyMapping))))
    (else
      (return (LocalVariables|GetbFound) (LocalVariables|GetKeyMapping)))))

(fn GetKeybindingName
  (params (Key :type Key%20Structure))
  (bind (_returnvalue _foundmapping) (Utility|DoesKeyExistinActionMapping Key))
  (bind (_returnvalue_2 _foundmapping_2) (Utility|DoesKeyExistinAxisMapping Key))
  (if _returnvalue
    (return (.ActionName (Utilities|Struct|BreakInputActionKeyMapping _foundmapping)))
    (elif _returnvalue_2
      (return (.AxisName (Utilities|Struct|BreakInputAxisKeyMapping _foundmapping_2)))
      (else
        (return "None")))))

(fn RebindActionMapping
  (params (KeymappingButton :type WB%20Button%2003%20Options%20Object%20Reference) (NewKey :type Key%20Structure))
  (bind _returnvalue (Class|InputSettings|GetInputSettings))
  ;[1 1 1] Set Data
  (LocalVariables|SetKey NewKey)
  (LocalVariables|SetRemoveOldMapping true)
  (Utilities|IsValid KeymappingButton
    (:Is%20Valid
      (LocalVariables|SetName (Variables|/Game/HQUI_Buttons/Widgets/Buttons/Button03/WB_Button03_Options.WB_Button03_Options_C|GetKeymappingName KeymappingButton))
      ;[1 1 1] Remove Mappings
      (if (LocalVariables|GetRemoveOldMapping)
        (|RemoveExistingActionMapping
          (:Completed
            (|RemoveActionMapping))))
      ;[1 1 1] Add Action Mapping
      (Class|InputSettings|AddActionMapping (Class|InputSettings|GetInputSettings) (Utilities|Struct|MakeInputActionKeyMapping (Utilities|String|StringToName (Utilities|String|ToString(Text) (LocalVariables|GetName))) false false false false (LocalVariables|GetKey)) true)
      ;[1 1 1] Apply Mappings
      (Class|InputSettings|ForceRebuildKeymaps _returnvalue)
      (Class|InputSettings|SaveKeyMappings _returnvalue)
      (return true))
    (:Is%20Not%20Valid
      (return false))))

(fn IsActionMapping
  (params (Key :type Key%20Structure))
  (LocalVariables|SetKeyTest Key)
  (for _array_element (Class|InputSettings|GetActionNames (Class|InputSettings|GetInputSettings))
    (bind _array_element_2 (Utilities|Array|ForEachLoopwithBreak (Class|InputSettings|GetActionMappingbyName (Class|InputSettings|GetInputSettings) _array_element) :!label _label)
      (:LoopBody
        (if (== (.Key (Utilities|Struct|BreakInputActionKeyMapping _array_element_2)) (LocalVariables|GetKeyTest))
          (LocalVariables|SetbIsAction true)
          (goto _label Break)))))
  (return (LocalVariables|GetbIsAction)))

(fn FindActionGamepadKey
  (params (InActionName :type Name))
  (bind _array_element (Utilities|Array|ForEachLoopwithBreak (Class|InputSettings|GetActionMappingbyName (Class|InputSettings|GetInputSettings) InActionName) :!label _label)
    (:LoopBody
      (if (Class|KismetInputLibrary|KeyIsGamepadKey (.Key (Utilities|Struct|BreakInputActionKeyMapping _array_element)))
        (LocalVariables|SetGamepadKey _array_element)
        (goto _label Break)))
    (:Completed
      (return (LocalVariables|GetGamepadKey)))))

(fn FindActionKeyboardMouseKey
  (params (InActionName :type Name))
  (bind _array_element (Utilities|Array|ForEachLoopwithBreak (Class|InputSettings|GetActionMappingbyName (Class|InputSettings|GetInputSettings) InActionName) :!label _label)
    (:LoopBody
      (if (or (Class|KismetInputLibrary|KeyIsKeyboardKey (.Key (Utilities|Struct|BreakInputActionKeyMapping _array_element))) (Class|KismetInputLibrary|KeyIsMouseButton (.Key (Utilities|Struct|BreakInputActionKeyMapping _array_element))))
        (LocalVariables|SetKeyboardMouseKey _array_element)
        (goto _label Break)))
    (:Completed
      (return (LocalVariables|GetKeyboardMouseKey)))))

(fn FindAxisGamepadKey
  (params (InAxisName :type Name))
  (bind _array_element (Utilities|Array|ForEachLoopwithBreak (Class|InputSettings|GetAxisMappingbyName (Class|InputSettings|GetInputSettings) InAxisName) :!label _label)
    (:LoopBody
      (if (Class|KismetInputLibrary|KeyIsGamepadKey (.Key (Utilities|Struct|BreakInputAxisKeyMapping _array_element)))
        (LocalVariables|SetGamepadKey _array_element)
        (goto _label Break)))
    (:Completed
      (return (LocalVariables|GetGamepadKey)))))

(fn FindAxisKeyboardMouseKey
  (params (InActionName :type Name))
  (bind _array_element (Utilities|Array|ForEachLoopwithBreak (Class|InputSettings|GetAxisMappingbyName (Class|InputSettings|GetInputSettings) InActionName) :!label _label)
    (:LoopBody
      (if (or (Class|KismetInputLibrary|KeyIsKeyboardKey (.Key (Utilities|Struct|BreakInputAxisKeyMapping _array_element))) (Class|KismetInputLibrary|KeyIsMouseButton (.Key (Utilities|Struct|BreakInputAxisKeyMapping _array_element))))
        (LocalVariables|SetKeyboardMouseKey _array_element)
        (goto _label Break)))
    (:Completed
      (return (LocalVariables|GetKeyboardMouseKey)))))

(fn RebindAxisMapping
  (params (KeymappingButton :type WB%20Button%2003%20Options%20Object%20Reference) (NewKey :type Key%20Structure))
  (bind _returnvalue (Class|InputSettings|GetInputSettings))
  ;[1 1 1] Set Data
  (LocalVariables|SetKey NewKey)
  (LocalVariables|SetRemoveOldMapping true)
  (Utilities|IsValid KeymappingButton
    (:Is%20Valid
      (LocalVariables|SetName (Variables|/Game/HQUI_Buttons/Widgets/Buttons/Button03/WB_Button03_Options.WB_Button03_Options_C|GetKeymappingName KeymappingButton))
      (LocalVariables|SetScale (|FindScale))
      ;[1 1 1] Remove Mappings
      (if (LocalVariables|GetRemoveOldMapping)
        (|RemoveExistingAxisMapping
          (:Completed
            (|RemoveAxisMapping))))
      ;[1 1 1] Add new Axis Mapping
      (Class|InputSettings|AddAxisMapping (Class|InputSettings|GetInputSettings) (Utilities|Struct|MakeInputAxisKeyMapping (Utilities|String|StringToName (Utilities|String|ToString(Text) (LocalVariables|GetName))) (LocalVariables|GetScale) (LocalVariables|GetKey)) true)
      ;[1 1 1] Apply Mappings
      (Class|InputSettings|ForceRebuildKeymaps _returnvalue)
      (Class|InputSettings|SaveKeyMappings _returnvalue)
      (return true))
    (:Is%20Not%20Valid
      (return false))))

(fn IsAnyGamepadThumbstick
  (params (Key :type Key%20Structure))
  (return (Math|Boolean|ORBoolean (== Key "Gamepad_LeftStick_Up") (== Key "Gamepad_LeftStick_Down") (== Key "Gamepad_LeftStick_Right") (== Key "Gamepad_LeftStick_Left") (== Key "Gamepad_RightStick_Up") (== Key "Gamepad_RightStick_Down") (== Key "Gamepad_RightStick_Right") (== Key "Gamepad_RightStick_Left"))))

(fn IsGamepadThumbstickL
  (params (Key :type Key%20Structure))
  (return (Math|Boolean|ORBoolean (== Key "Gamepad_LeftStick_Up") (== Key "Gamepad_LeftStick_Down") (== Key "Gamepad_LeftStick_Right") (== Key "Gamepad_LeftStick_Left"))))

(fn IsGamepadThumbstickLXAxis
  (params (Key :type Key%20Structure))
  (return (or (== Key "Gamepad_LeftStick_Right") (== Key "Gamepad_LeftStick_Left"))))

(fn IsGamepadThumbstickLYAxis
  (params (Key :type Key%20Structure))
  (return (or (== Key "Gamepad_LeftStick_Up") (== Key "Gamepad_LeftStick_Down"))))

(fn IsGamepadThumbstickR
  (params (Key :type Key%20Structure))
  (return (Math|Boolean|ORBoolean (== Key "Gamepad_RightStick_Up") (== Key "Gamepad_RightStick_Down") (== Key "Gamepad_RightStick_Right") (== Key "Gamepad_RightStick_Left"))))

(fn IsGamepadThumbstickRXAxis
  (params (Key :type Key%20Structure))
  (return (or (== Key "Gamepad_RightStick_Right") (== Key "Gamepad_RightStick_Left"))))

(fn IsGamepadThumbstickRYAxis
  (params (Key :type Key%20Structure))
  (return (or (== Key "Gamepad_RightStick_Up") (== Key "Gamepad_RightStick_Down"))))

(fn UseRebindXandYAxis
  (params (Key :type Key%20Structure) (UseRebindX_And_Y_Axis :type Boolean))
  (return (select (and (Utility|Rebinding|IsGamepadThumbstickLXAxis 0 Key) UseRebindX_And_Y_Axis) "Gamepad_LeftX" (select (and (Utility|Rebinding|IsGamepadThumbstickLYAxis 0 Key) UseRebindX_And_Y_Axis) "Gamepad_LeftY" (select (and (Utility|Rebinding|IsGamepadThumbstickRXAxis 0 Key) UseRebindX_And_Y_Axis) "Gamepad_RightX" (select (and (Utility|Rebinding|IsGamepadThumbstickRYAxis 0 Key) UseRebindX_And_Y_Axis) "Gamepad_RightY" Key))))))