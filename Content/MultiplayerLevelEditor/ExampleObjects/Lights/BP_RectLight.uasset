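; BP_RectLight is an example rect light object for the multiplayer level editor, implementing the editor's callbacks for scaling, material, selection, grab, release and delete.
; Scale and material events set RepNotify variables, whose OnRep functions apply the actor scale and material item.
; Selectability changes only on the authority and is read through CanSelect.
; Grab, release and delete events are empty, debug prints are unwired, and property getters return nothing.
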(event EventBeginPlay)

(event Collision|EventActorBeginOverlap
  (params (OtherActor :type Actor%20Object%20Reference)))

(event EventOnRelease)

(event EventOnMaterialLoaded
  (params (MapEditorItemMaterial :type SKGMLE%20Item%20Material%20Data%20Structure%20%28by%20ref%29))
  (Variables|Default|SetMap%20Editor%20Item%20Material MapEditorItemMaterial))

(event EventOnGrabbed)

(event EventOnDeleted)

(event EventOnScaleChanged
  (params (NewScale :type Vector :default "0, 0, 0"))
  (Variables|Default|SetScale NewScale))

(event EventTick
  (params (DeltaSeconds :type Float%20%28single-precision%29)))

(event EventSetCanSelect
  (params (bCanSelect :type Boolean))
  (Networking|SwitchHasAuthority
    (:Authority
      (Variables|Default|SetbCanSelect bCanSelect))))

(fn ConstructionScript)

(fn OnRepScale
  (Transformation|SetActorScale3D (Variables|Default|GetScale)))

(fn OnRepMapEditorItemMaterial
  (Class|SKGMLEStatics|ApplyMaterialItem (Variables|Default|GetMap%20Editor%20Item%20Material)))

(fn CanSelect
  (return (Variables|Default|GetbCanSelect)))

(fn GetAllBoolProperties
  (return 0))

(fn GetAllFloatProperties
  (return 0))

(fn GetAllIntProperties
  (return 0))

(fn GetAllNameProperties
  (return 0))

(fn GetAllStringProperties
  (return 0))

(fn GetAllTextProperties
  (return 0))